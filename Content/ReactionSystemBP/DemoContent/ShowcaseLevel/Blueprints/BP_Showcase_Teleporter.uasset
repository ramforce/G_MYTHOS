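; Showcase-level teleporter that moves the player character to the location and rotation of its Destination component when they overlap the CollisionTrigger.
; A separate TextCollisionBox controls a text label that starts at zero scale on BeginPlay.
; Entering the box shows the text and grows it to DesiredWorldScale through a timeline lerp, while leaving plays a second timeline that shrinks it and then hides it.
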(event OnComponentBeginOverlap(CollisionTrigger)
  (params (OverlappedComponent :type Primitive%20Component%20Object%20Reference) (OtherActor :type Actor%20Object%20Reference) (OtherComp :type Primitive%20Component%20Object%20Reference) (OtherBodyIndex :type Integer) (bFromSweep :type Boolean) (SweepResult :type Hit%20Result%20Structure%20%28by%20ref%29))
  (if (== OtherActor (Game|GetPlayerCharacter 0))
    (Variables|Default|SetTargetToTeleport OtherActor)
    (CallFunction|TeleportPlayertoLocation)))

(event OnComponentBeginOverlap(TextCollisionBox)
  (params (OverlappedComponent :type Primitive%20Component%20Object%20Reference) (OtherActor :type Actor%20Object%20Reference) (OtherComp :type Primitive%20Component%20Object%20Reference) (OtherBodyIndex :type Integer) (bFromSweep :type Boolean) (SweepResult :type Hit%20Result%20Structure%20%28by%20ref%29))
  (if (== OtherActor (Game|GetPlayerCharacter 0))
    (CallFunction|PlayScalingTimeline)))

(event OnComponentEndOverlap(TextCollisionBox)
  (params (OverlappedComponent :type Primitive%20Component%20Object%20Reference) (OtherActor :type Actor%20Object%20Reference) (OtherComp :type Primitive%20Component%20Object%20Reference) (OtherBodyIndex :type Integer))
  (if (== OtherActor (Game|GetPlayerCharacter 0))
    (CallFunction|ReverseScalingTimeline)))

(event Custom|TeleportPlayerToLocation
  (bind _destination (Variables|Default|GetDestination))
  (Transformation|Teleport (Variables|Default|GetTargetToTeleport) (Transformation|GetWorldLocation _destination) (Transformation|GetWorldRotation _destination)))

(event Custom|PlayScalingTimeline
  (Rendering|SetVisibility (Variables|Default|GetTextRender) true false)
  (bind _alpha (Timeline|Timeline_0 PlayFromStart)
    (:Update
      (Transformation|SetWorldScale3D (Variables|Default|GetTextRender) (Math|Vector|Lerp(Vector) "0, 0, 0" (Variables|Default|GetDesiredWorldScale) _alpha)))))

(event Custom|ReverseScalingTimeline
  (bind _alpha (Timeline|Timeline_1 PlayFromStart)
    (:Update
      (Transformation|SetWorldScale3D (Variables|Default|GetTextRender) (Math|Vector|Lerp(Vector) (Variables|Default|GetDesiredWorldScale) "0, 0, 0" _alpha)))
    (:Finished
      (Rendering|SetVisibility (Variables|Default|GetTextRender) false false))))

(event EventBeginPlay
  (Transformation|SetWorldScale3D (Variables|Default|GetTextRender) "0, 0, 0"))

(fn ConstructionScript)