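; Showcase level title actor that reveals 3D text and a point light while something overlaps its trigger.
; Begin overlap shows both and plays a timeline that lerps text world size and light intensity from zero to the desired values.
; If ShouldFadeAwayInstantly is set, end overlap waits FadeDelay, then a second timeline shrinks and dims them, hides them and optionally destroys the actor.
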(event OnComponentBeginOverlap(OverlapTrigger)
  (params (OverlappedComponent :type Primitive%20Component%20Object%20Reference) (OtherActor :type Actor%20Object%20Reference) (OtherComp :type Primitive%20Component%20Object%20Reference) (OtherBodyIndex :type Integer) (bFromSweep :type Boolean) (SweepResult :type Hit%20Result%20Structure%20%28by%20ref%29))
  (CallFunction|PlayScalingTimeline)
  (Rendering|SetVisibility (Variables|Default|GetTextRender) true false)
  (Development|SetHiddeninGame (Variables|Default|GetPointLight) false false))

(event OnComponentEndOverlap(OverlapTrigger)
  (params (OverlappedComponent :type Primitive%20Component%20Object%20Reference) (OtherActor :type Actor%20Object%20Reference) (OtherComp :type Primitive%20Component%20Object%20Reference) (OtherBodyIndex :type Integer))
  (if (Variables|Default|GetShould%20Fade%20Away%20Instantly?)
    (Utilities|FlowControl|Delay (Variables|Default|GetFadeDelay))
    (CallFunction|ReverseScalingTimeline)))

(event Custom|PlayScalingTimeline
  (bind _alpha (Timeline|AlphaTimeline PlayFromStart)
    (:Update
      (Rendering|Components|TextRender|SetWorldSize (Variables|Default|GetTextRender) (Math|Float|Lerp 0.0 (Variables|Default|GetDesiredWorldScale) _alpha))
      (Rendering|Components|Light|SetIntensity (Variables|Default|GetPointLight) (Math|Float|Lerp 0.0 (Variables|Default|GetDesiredIntensity) _alpha)))))

(event Custom|ReverseScalingTimeline
  (bind _alpha (Timeline|Timeline_0 PlayFromStart)
    (:Update
      (Rendering|Components|TextRender|SetWorldSize (Variables|Default|GetTextRender) (Math|Float|Lerp (Variables|Default|GetDesiredWorldScale) 0.0 _alpha))
      (Rendering|Components|Light|SetIntensity (Variables|Default|GetPointLight) (Math|Float|Lerp (Variables|Default|GetDesiredIntensity) 0.0 _alpha)))
    (:Finished
      (Rendering|SetVisibility (Variables|Default|GetTextRender) false false)
      (Development|SetHiddeninGame (Variables|Default|GetPointLight) true false)
      (if (Variables|Default|GetShouldDelete?)
        (Actor|DestroyActor)))))

(event EventBeginPlay
  (Rendering|Components|TextRender|SetWorldSize (Variables|Default|GetTextRender) 0.0))

(fn ConstructionScript)