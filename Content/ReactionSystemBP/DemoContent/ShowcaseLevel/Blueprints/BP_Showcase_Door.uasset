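; Showcase level sliding double door that opens when an actor enters its overlap trigger and closes when one leaves.
; BeginPlay caches each panel's closed location and an open location offset sideways along its right vector.
; Overlap events call OpenDoor and CloseDoor, which play or reverse the DoorOpening timeline to lerp both panels apart or back.
; The player-only checks and instant teleport moves are disconnected, so overlaps are not filtered by actor.
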(event OnComponentEndOverlap(OverlapTrigger)
  (params (OverlappedComponent :type Primitive%20Component%20Object%20Reference) (OtherActor :type Actor%20Object%20Reference) (OtherComp :type Primitive%20Component%20Object%20Reference) (OtherBodyIndex :type Integer))
  (CallFunction|CloseDoor))

(event OnComponentBeginOverlap(OverlapTrigger)
  (params (OverlappedComponent :type Primitive%20Component%20Object%20Reference) (OtherActor :type Actor%20Object%20Reference) (OtherComp :type Primitive%20Component%20Object%20Reference) (OtherBodyIndex :type Integer) (bFromSweep :type Boolean) (SweepResult :type Hit%20Result%20Structure%20%28by%20ref%29))
  (CallFunction|OpenDoor))

(event Custom|CustomEvent_1
  (bind _alpha (Timeline|DoorOpening Reverse)
    (:Update
      (Transformation|SetWorldLocation (Variables|Default|GetDoor_left) (Math|Vector|Lerp(Vector) (Variables|Default|GetLeftDoorDefaultLoc) (Variables|Default|GetLeftDoorDesiredLoc) _alpha) false false)
      (Transformation|SetWorldLocation (Variables|Default|GetDoor_right) (Math|Vector|Lerp(Vector) (Variables|Default|GetRightDoorDefaultLoc) (Variables|Default|GetRightDoorDesiredLoc) _alpha) false false))))

(event Custom|CustomEvent
  (bind _alpha (Timeline|DoorOpening Play)
    (:Update
      (Transformation|SetWorldLocation (Variables|Default|GetDoor_left) (Math|Vector|Lerp(Vector) (Variables|Default|GetLeftDoorDefaultLoc) (Variables|Default|GetLeftDoorDesiredLoc) _alpha) false false)
      (Transformation|SetWorldLocation (Variables|Default|GetDoor_right) (Math|Vector|Lerp(Vector) (Variables|Default|GetRightDoorDefaultLoc) (Variables|Default|GetRightDoorDesiredLoc) _alpha) false false))))

(event Custom|OpenDoor
  (CallFunction|CustomEvent))

(event Custom|CloseDoor
  (CallFunction|CustomEvent1))

(event EventBeginPlay
  (bind _door_left (Variables|Default|GetDoor_left))
  (bind _door_right (Variables|Default|GetDoor_right))
  (Variables|Default|SetLeftDoorDefaultLoc (Transformation|GetWorldLocation (Variables|Default|GetDoor_left)))
  (Variables|Default|SetRightDoorDefaultLoc (Transformation|GetWorldLocation (Variables|Default|GetDoor_right)))
  (Variables|Default|SetLeftDoorDesiredLoc (+ (Transformation|GetWorldLocation _door_left) (* (Math|Vector|GetRightVector _door_left) 2.5e+02)))
  (Variables|Default|SetRightDoorDesiredLoc (+ (Transformation|GetWorldLocation _door_right) (* (* (Math|Vector|GetRightVector _door_right) 2.5e+02) -1.0))))

(fn ConstructionScript)