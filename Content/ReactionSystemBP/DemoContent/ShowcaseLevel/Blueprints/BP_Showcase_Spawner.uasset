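; Showcase level spawner that lets the player spawn an AI pawn of a configurable class by pressing E while near it.
; An overlap trigger enables and disables the actor's input as the player character enters and leaves.
; Timelines scale a text render in on entry and out on exit or key press, hiding it afterwards.
; The pawn spawns at an arrow component's location, using only its yaw.
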(event OnComponentBeginOverlap(OverlapTrigger)
  (params (OverlappedComponent :type Primitive%20Component%20Object%20Reference) (OtherActor :type Actor%20Object%20Reference) (OtherComp :type Primitive%20Component%20Object%20Reference) (OtherBodyIndex :type Integer) (bFromSweep :type Boolean) (SweepResult :type Hit%20Result%20Structure%20%28by%20ref%29))
  (if (== OtherActor (Game|GetPlayerCharacter 0))
    (Input|EnableInput (Game|GetPlayerController 0))
    (CallFunction|PlayScalingTimeline)))

(event OnComponentEndOverlap(OverlapTrigger)
  (params (OverlappedComponent :type Primitive%20Component%20Object%20Reference) (OtherActor :type Actor%20Object%20Reference) (OtherComp :type Primitive%20Component%20Object%20Reference) (OtherBodyIndex :type Integer))
  (if (== OtherActor (Game|GetPlayerCharacter 0))
    (Input|DisableInput (Game|GetPlayerController 0))
    (if (Rendering|IsVisible (Variables|Default|GetTextRender))
      (CallFunction|ReverseScalingTimeline))))

(event Custom|PlayScalingTimeline
  (Rendering|SetVisibility (Variables|Default|GetTextRender) true false)
  (bind _alpha (Timeline|Timeline_0 PlayFromStart)
    (:Update
      (Transformation|SetWorldScale3D (Variables|Default|GetTextRender) (Math|Vector|Lerp(Vector) "0, 0, 0" (Variables|Default|GetDesiredWorldScale) _alpha)))))

(event Custom|ReverseScalingTimeline
  (bind _alpha (Timeline|Timeline_1 PlayFromStart)
    (:Update
      (Transformation|SetWorldScale3D (Variables|Default|GetTextRender) (Math|Vector|Lerp(Vector) (Variables|Default|GetDesiredWorldScale) "0, 0, 0" _alpha)))
    (:Finished
      (Rendering|SetVisibility (Variables|Default|GetTextRender) false false))))

(event EventBeginPlay)

(event Collision|EventActorBeginOverlap
  (params (OtherActor :type Actor%20Object%20Reference)))

(event EventTick
  (params (DeltaSeconds :type Float%20%28single-precision%29)))

(event Input|KeyboardEvents|E
  (params (Key :type Key%20Structure))
  (bind _arrow (Variables|Default|GetArrow))
  (:Pressed
    (AI|SpawnAIFromClass (Variables|Default|GetActorToSpawn) 0 (Transformation|GetWorldLocation _arrow) (Math|Rotator|MakeRotator 0.0 0.0 (.Yaw (Math|Rotator|BreakRotator (Transformation|GetWorldRotation _arrow)))) false)
    (if (Rendering|IsVisible (Variables|Default|GetTextRender))
      (CallFunction|ReverseScalingTimeline))))

(fn ConstructionScript)