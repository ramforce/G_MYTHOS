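; Showcase info platform for the Reaction System demo level that displays a chosen Paper sprite and lets the player focus the camera on it.
; When the player character enters the overlap trigger, input is enabled and a text prompt scales in via timeline.
; The Interact input toggles a blended view target between this actor and the previous one, hiding the prompt while focused.
; Leaving disables input, scales out the visible prompt and exits focus.
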(event OnComponentBeginOverlap(OverlapTrigger)
  (params (OverlappedComponent :type Primitive%20Component%20Object%20Reference) (OtherActor :type Actor%20Object%20Reference) (OtherComp :type Primitive%20Component%20Object%20Reference) (OtherBodyIndex :type Integer) (bFromSweep :type Boolean) (SweepResult :type Hit%20Result%20Structure%20%28by%20ref%29))
  (if (== OtherActor (Game|GetPlayerCharacter 0))
    (Input|EnableInput (Game|GetPlayerController 0))
    (CallFunction|PlayScalingTimeline)))

(event OnComponentEndOverlap(OverlapTrigger)
  (params (OverlappedComponent :type Primitive%20Component%20Object%20Reference) (OtherActor :type Actor%20Object%20Reference) (OtherComp :type Primitive%20Component%20Object%20Reference) (OtherBodyIndex :type Integer))
  (if (== (stale OnComponentBeginOverlap(OverlapTrigger) OtherActor) (Game|GetPlayerCharacter 0))
    (Input|DisableInput (Game|GetPlayerController 0))
    (if (Rendering|IsVisible (Variables|Default|GetTextRender))
      (CallFunction|ReverseScalingTimeline))
    (if (Variables|Default|GetIsImageFocused?)
      (CallFunction|TogglePlayerViewTarget false))))

(event Custom|TogglePlayerViewTarget
  (params (FocusImage? :type Boolean))
  (bind _returnvalue (Game|GetPlayerController 0))
  (if FocusImage?
    (Variables|Default|SetIsImageFocused? true)
    (Variables|Default|SetPreviousViewTarget (Pawn|GetViewTarget _returnvalue))
    (Game|Player|SetViewTargetwithBlend _returnvalue self 1.0 "VTBlend_Linear" 0.0 false)
    (Rendering|SetVisibility (Variables|Default|GetTextRender) false false)
    (else
      (Variables|Default|SetIsImageFocused? false)
      (Game|Player|SetViewTargetwithBlend _returnvalue (Variables|Default|GetPreviousViewTarget) 1.0 "VTBlend_Linear" 0.0 false)
      (Rendering|SetVisibility (Variables|Default|GetTextRender) true false))))

(event Custom|PlayScalingTimeline
  (Rendering|SetVisibility (Variables|Default|GetTextRender) true false)
  (bind _alpha (Timeline|Timeline_0 PlayFromStart)
    (:Update
      (Transformation|SetWorldScale3D (Variables|Default|GetTextRender) (Math|Vector|Lerp(Vector) "0, 0, 0" (Variables|Default|GetDesiredWorldScale) _alpha)))))

(event Custom|ReverseScalingTimeline
  (bind _alpha (Timeline|Timeline_1 PlayFromStart)
    (:Update
      (Transformation|SetWorldScale3D (Variables|Default|GetTextRender) (Math|Vector|Lerp(Vector) (Variables|Default|GetDesiredWorldScale) "0, 0, 0" _alpha)))
    (:Finished
      (Rendering|SetVisibility (Variables|Default|GetTextRender) false false))))

(event Input|ActionEvents|InputActionInteract
  (params (Key :type Key%20Structure))
  (:Pressed
    (if (Variables|Default|GetIsImageFocused?)
      (CallFunction|TogglePlayerViewTarget false)
      (else
        (CallFunction|TogglePlayerViewTarget true)))))

(fn ConstructionScript
  (Rendering|Components|Sprite|SetSprite (Variables|Default|GetPaperSprite) (Variables|Default|GetSpriteToDisplay)))