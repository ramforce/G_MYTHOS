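; BP_Showcase_Board is an info board actor for the Reaction System showcase level that displays a title and a description.
; Its construction script copies the text and world size variables into the TitleText and DescriptionText components, so each placed board is configured per instance.
; It has no active event logic, and a cull distance call on both texts is left unconnected.
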(event EventBeginPlay)

(event Collision|EventActorBeginOverlap
  (params (OtherActor :type Actor%20Object%20Reference)))

(event EventTick
  (params (DeltaSeconds :type Float%20%28single-precision%29)))

(fn ConstructionScript
  (Rendering|Components|TextRender|SetText (Variables|Default|GetTitle%20Text) (Variables|TitleSetup|GetTitleTextValue))
  (Rendering|Components|TextRender|SetWorldSize (Variables|Default|GetTitle%20Text) (Variables|TitleSetup|GetTitleTextWorldSize))
  (Rendering|Components|TextRender|SetText (Variables|Default|GetDescription%20Text) (Variables|DescriptionSetup|GetDescriptionTextValue))
  (Rendering|Components|TextRender|SetWorldSize (Variables|Default|GetDescription%20Text) (Variables|DescriptionSetup|GetDescriptionTextWorldSize)))