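; Showcase level info platform that displays text, optionally hidden until the player presses Interact inside its overlap trigger.
; Each press sets the next entry from paired info arrays, wrapping around, and plays a timeline that scales the text up.
; When text is not hidden, the button mesh is destroyed at start.
; Construction either adds a styled title or, without one, picks the platform mesh and optional emissive border color.
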(event OnComponentBeginOverlap(OverlapTrigger)
  (params (OverlappedComponent :type Primitive%20Component%20Object%20Reference) (OtherActor :type Actor%20Object%20Reference) (OtherComp :type Primitive%20Component%20Object%20Reference) (OtherBodyIndex :type Integer) (bFromSweep :type Boolean) (SweepResult :type Hit%20Result%20Structure%20%28by%20ref%29))
  (if (== OtherActor (Game|GetPlayerCharacter 0))
    (Input|EnableInput (Game|GetPlayerController 0))))

(event OnComponentEndOverlap(OverlapTrigger)
  (params (OverlappedComponent :type Primitive%20Component%20Object%20Reference) (OtherActor :type Actor%20Object%20Reference) (OtherComp :type Primitive%20Component%20Object%20Reference) (OtherBodyIndex :type Integer))
  (if (== (stale OnComponentBeginOverlap(OverlapTrigger) OtherActor) (Game|GetPlayerCharacter 0))
    (Input|DisableInput (Game|GetPlayerController 0))))

(event Custom|Select%20New%20Info%20Text
  (Rendering|Components|TextRender|SetText (Variables|Default|GetTextRender) (Utilities|Text|FormatText "{wrap} 
{wrapb}" (Utilities|Array|Get(acopy) (Variables|Default|GetInfoArray) (Variables|Default|GetInfoIndex)) (Utilities|Array|Get(acopy) (Variables|Default|GetInfoArray_Line1) (Variables|Default|GetInfoIndex))))
  (if (>= (Variables|Default|GetInfoIndex) (- (Utilities|Array|Length (Variables|Default|GetInfoArray)) 1))
    (Variables|Default|SetInfoIndex 0)
    (else
      (Variables|Default|SetInfoIndex (+ (Variables|Default|GetInfoIndex) 1))))
  (Development|PrintString (Utilities|String|ToString(Integer) (Variables|Default|GetInfoIndex))))

(event Custom|PlayScalingTimeline
  (bind _alpha (Timeline|Timeline_0 PlayFromStart)
    (:Update
      (Transformation|SetWorldScale3D (Variables|Default|GetTextRender) (Math|Vector|Lerp(Vector) "0, 0, 0" (Variables|Default|GetDesiredWorldScale) _alpha)))))

(event Custom|ReverseScalingTimeline
  (Timeline|Timeline_1 PlayFromStart
    (:Update
      (Transformation|SetWorldScale3D (Variables|Default|GetTextRender) (Math|Vector|Lerp(Vector) (Variables|Default|GetDesiredWorldScale) "0, 0, 0" 0.0)))
    (:Finished
      (Rendering|SetVisibility (Variables|Default|GetTextRender) false false))))

(event EventBeginPlay
  (if (Variables|Text|GetShouldHideShowcaseText?)
    (Transformation|SetWorldScale3D (Variables|Default|GetTextRender) "0, 0, 0")
    (else
      (Components|DestroyComponent (Variables|Default|GetButtonMesh)))))

(event Input|ActionEvents|InputActionInteract
  (params (Key :type Key%20Structure))
  (:Pressed
    (if (Variables|Text|GetShouldHideShowcaseText?)
      (CallFunction|SelectNewInfoText)
      (CallFunction|PlayScalingTimeline))))

(fn ConstructionScript
  (bind _platformmesh (Variables|Default|GetPlatformMesh))
  (bind _platformmesh_2 (Variables|Default|GetPlatformMesh))
  (if (Variables|Title|GetHasTitle?)
    (bind _returnvalue (AddComponent|AddTextRenderComponent false (Transformation|GetRelativeTransform (Variables|Default|GetArrow))))
    (Transformation|SetWorldScale3D _returnvalue (Variables|Title|GetDesiredTitleSize))
    (Rendering|Components|TextRender|SetTextRenderColor _returnvalue (Variables|Title|GetTitleColor))
    (Rendering|Components|TextRender|SetText _returnvalue (Variables|Title|GetTitleText))
    (else
      (switch int (Variables|Default|GetPlatformType)
        (:Default
          (Components|StaticMesh|SetStaticMesh _platformmesh "/Game/ReactionSystemBP/DemoContent/ShowcaseLevel/DemoRoom/Meshes/SM_Base.SM_Base" :!label _label))
        (:1
          (goto _label))
        (:2
          (Components|StaticMesh|SetStaticMesh _platformmesh "/Game/ReactionSystemBP/DemoContent/ShowcaseLevel/DemoRoom/Meshes/SM_Base2.SM_Base2"))
        (:3
          (Components|StaticMesh|SetStaticMesh _platformmesh "/Game/ReactionSystemBP/DemoContent/ShowcaseLevel/DemoRoom/Meshes/SM_Base_FlatWall.SM_Base_FlatWall")))
      (if (Variables|Default|GetEmissiveBorders?)
        (switch int (Variables|Default|GetEmissiveColorIndex)
          (:1
            (Rendering|Material|SetMaterial _platformmesh_2 2 "/Game/ReactionSystemBP/DemoContent/ShowcaseLevel/DemoRoom/Materials/M_Showcase_Emissive_Green.M_Showcase_Emissive_Green"))
          (:2
            (Rendering|Material|SetMaterial _platformmesh_2 2 "/Game/ReactionSystemBP/DemoContent/ShowcaseLevel/DemoRoom/Materials/M_Showcase_Emissive_Red.M_Showcase_Emissive_Red"))
          (:3
            (Rendering|Material|SetMaterial _platformmesh_2 2 "/Game/ReactionSystemBP/DemoContent/ShowcaseLevel/DemoRoom/Materials/M_Showcase_Emissive_Blue.M_Showcase_Emissive_Blue")))))))