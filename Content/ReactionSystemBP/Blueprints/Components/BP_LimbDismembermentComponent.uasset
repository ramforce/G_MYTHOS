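; Actor component that dismembers a character's head, arms or legs after enough hits on that limb.
; SetCurrentLimbIndex maps a hit bone to a limb, then IncrementHitCounterOnLimb updates its counter and checks threshold and dismemberable flag.
; Dismemberment hides the bone, plays burst and attached bleeding emitters, and launches a fake BP_LimbActor_Master limb.
; Server/Multicast-named events drive effects, with optional owner kill or custom reaction via messages.
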(event Custom|Multicast%20Start%20Limb%20Dismemberment
  (bind _ownermesh (Variables|Default|GetOwnerMesh))
  (bind _bonenamestructure (Variables|DismembermentSetup|GetBoneNameStructure))
  (bind _ownermesh_2 (Variables|Default|GetOwnerMesh))
  (bind _bonenamestructure_2 (Variables|DismembermentSetup|GetBoneNameStructure))
  (bind _ownermesh_3 (Variables|Default|GetOwnerMesh))
  (bind _dismemberedlimbindex (Variables|Don'tTouch|GetDismemberedLimbIndex))
  (bind _bonenamestructure_3 (Variables|DismembermentSetup|GetBoneNameStructure))
  (bind _dismembermentemitter (Variables|DismembermentEmitterSetup|GetDismembermentEmitter))
  (bind _dismembermentemitter_2 (Variables|DismembermentEmitterSetup|GetDismembermentEmitter))
  (bind _limbarrayindex (Variables|DismembermentSetup|GetLimbArrayIndex))
  (bind _dismembermentemitter_3 (Variables|DismembermentEmitterSetup|GetDismembermentEmitter))
  (bind _ownermesh_4 (Variables|Default|GetOwnerMesh))
  (bind _dismembermentemitter_4 (Variables|DismembermentEmitterSetup|GetDismembermentEmitter))
  (bind _dismembermentemitter_5 (Variables|DismembermentEmitterSetup|GetDismembermentEmitter))
  (bind _bonenamestructure_4 (Variables|DismembermentSetup|GetBoneNameStructure))
  (bind _ownermesh_5 (Variables|Default|GetOwnerMesh))
  (bind _bonenamestructure_5 (Variables|DismembermentSetup|GetBoneNameStructure))
  (bind (_emittertoplay _emitterrotation _emitterscale) (Utilities|Struct|BreakS_ReactionEmitterInfo _dismembermentemitter))
  (bind _leftthighbone (Utilities|Struct|BreakS_BoneNames _bonenamestructure_2))
  (bind (_headindex _rightarmindex _leftarmindex _rightlegindex _leftlegindex) (Utilities|Struct|BreakS_LimbArrayIndex _limbarrayindex))
  (bind _headbone (Utilities|Struct|BreakS_BoneNames _bonenamestructure_3))
  (bind (_emittertoplay_2 _emitterrotation_2 _emitterscale_2) (Utilities|Struct|BreakS_ReactionEmitterInfo _dismembermentemitter_2))
  (bind (_emittertoplay_3 _emitterrotation_3 _emitterscale_3) (Utilities|Struct|BreakS_ReactionEmitterInfo _dismembermentemitter_3))
  (bind (_emittertoplay_4 _emitterrotation_4 _emitterscale_4) (Utilities|Struct|BreakS_ReactionEmitterInfo _dismembermentemitter_4))
  (bind (_emittertoplay_5 _emitterrotation_5 _emitterscale_5) (Utilities|Struct|BreakS_ReactionEmitterInfo _dismembermentemitter_5))
  (bind _rightthighbone (Utilities|Struct|BreakS_BoneNames _bonenamestructure_4))
  (bind _rightupperarmbone (Utilities|Struct|BreakS_BoneNames _bonenamestructure_5))
  (bind _leftupperarmbone (Utilities|Struct|BreakS_BoneNames _bonenamestructure))
  (bind _returnvalue (Transformation|GetSocketLocation _ownermesh _rightupperarmbone))
  (bind _returnvalue_2 (Transformation|GetSocketLocation _ownermesh_4 _headbone))
  (bind _returnvalue_3 (Transformation|GetSocketLocation _ownermesh_2 _leftupperarmbone))
  (bind _returnvalue_4 (Transformation|GetSocketLocation _ownermesh_5 _rightthighbone))
  (bind _returnvalue_5 (Transformation|GetSocketLocation _ownermesh_3 _leftthighbone))
  ;[1 1 1] Start Limb Dismemberment - The main event of the dismemberment component - hides dismembered bone, spawns emitters, spawn fake limb
  ;;[0 0.5355 1] Select which code to play, based on the "DismemberedLimbIndex"(gets set in CheckHitsOnLimb event)
  (if (== _headindex _dismemberedlimbindex)
    ;;[0 0.1294 0.2431] Head Dismemberment Logic
    ;;;[0 0.5355 1] Check if the bone is hidden already (it's already dismembered)
    (bind _returnvalue_6 (Class|SkinnedMeshComponent|IsBoneHiddenbyName (Variables|Default|GetOwnerMesh) _headbone))
    (if (not _returnvalue_6)
      ;;;[0 0.5355 1] If it's not dismembered, then dismember it by hiding the selected bone, and spawning the selected ReactionEmitter.
      (Components|SkinnedMesh|HideBonebyName _ownermesh_4 _headbone "PBO_None")
      (CallFunction|ServerSpawnEmitteratLocation _emittertoplay_2 _returnvalue_2 _emitterrotation_2 _emitterscale_2)
      ;;;[0 0.5355 1] After hiding the bone, spawn the fake limb actor (that's falling down to the floor) using the SpawnDismemberedActor event.
      (CallFunction|SpawnDismemberedActor (.HeadMesh (Utilities|Struct|BreakS_LimbActors (Variables|DismembermentSetup|GetLimbActorsToSpawn))) (Math|Transform|MakeTransform _returnvalue_2 (Transformation|GetSocketRotation (Variables|Default|GetOwnerMesh) _headbone)))
      ;;;[0 0.5355 1] Then spawn the attached emitter (to fake continous bleeding from the source) to the bone that's been hidden.
      (Effects|SpawnEmitterAttached (Variables|DismembermentEmitterSetup|GetLimbAttachedEmitter) (Variables|Default|GetOwnerMesh) (.HeadSocketName (Utilities|Struct|BreakS_LimbSocketNames (Variables|DismembermentSetup|GetLimbSocketNames))) "0, 0, 0" (.HeadEmitterRotation (Utilities|Struct|BreakS_DismemberedEmitterRotations (Variables|DismembermentEmitterSetup|GetAttachedEmitterRotations))))
      ;;;[0 0.5355 1] If the head is dismembered, check if the HeadDismemberedKillActor == true. If it is, send the InstantKill message to the owner.
      (if (not (Variables|DismembermentSetup|GetShouldKillOnAnyDismemberment?))
        (if (Variables|DismembermentSetup|GetHeadDismemberedKillActor?)
          (Class|BPIReactionComponent|InstantKillOwner(Message) (Components|GetOwner)))))
    (elif (== _rightarmindex _dismemberedlimbindex)
      ;;[0 0.1294 0.2431] Right Arm Dismemberment Logic
      ;;;[0 0.5355 1] Check if the bone is hidden already (it's already dismembered)
      (bind _returnvalue_7 (Class|SkinnedMeshComponent|IsBoneHiddenbyName (Variables|Default|GetOwnerMesh) _rightupperarmbone))
      (if (not _returnvalue_7)
        ;;;[0 0.5355 1] If it's not dismembered, then dismember it by hiding the selected bone, and spawning the selected ReactionEmitter.
        (Components|SkinnedMesh|HideBonebyName _ownermesh _rightupperarmbone "PBO_None")
        (CallFunction|ServerSpawnEmitteratLocation _emittertoplay_3 _returnvalue _emitterrotation_3 _emitterscale_3)
        ;;;[0 0.5355 1] After hiding the bone, spawn the fake limb actor (that's falling down to the floor) using the SpawnDismemberedActor event.
        (CallFunction|SpawnDismemberedActor (.RightArmMesh (Utilities|Struct|BreakS_LimbActors (Variables|DismembermentSetup|GetLimbActorsToSpawn))) (Math|Transform|MakeTransform _returnvalue (Math|Rotator|MakeRotator 0.0 0.0 (.Yaw (Math|Rotator|BreakRotator (Transformation|GetSocketRotation (Variables|Default|GetOwnerMesh) _rightupperarmbone))))))
        ;;;[0 0.5355 1] Then spawn the attached emitter (to fake continous bleeding from the source) to the bone that's been hidden.
        (Effects|SpawnEmitterAttached (Variables|DismembermentEmitterSetup|GetLimbAttachedEmitter) (Variables|Default|GetOwnerMesh) (.RightUpperArmSocketName (Utilities|Struct|BreakS_LimbSocketNames (Variables|DismembermentSetup|GetLimbSocketNames))) "0, 0, 0" (.RigtArmEmitterRotation (Utilities|Struct|BreakS_DismemberedEmitterRotations (Variables|DismembermentEmitterSetup|GetAttachedEmitterRotations)))))
      (elif (== _leftarmindex _dismemberedlimbindex)
        ;;[0 0.1294 0.2431] Left Arm Dismemberment Logic
        ;;;[0 0.5355 1] Check if the bone is hidden already (it's already dismembered)
        (bind _returnvalue_8 (Class|SkinnedMeshComponent|IsBoneHiddenbyName (Variables|Default|GetOwnerMesh) _leftupperarmbone))
        (if (not _returnvalue_8)
          ;;;[0 0.5355 1] If it's not dismembered, then dismember it by hiding the selected bone, and spawning the selected ReactionEmitter.
          (Components|SkinnedMesh|HideBonebyName _ownermesh_2 _leftupperarmbone "PBO_None")
          (CallFunction|ServerSpawnEmitteratLocation _emittertoplay_4 _returnvalue_3 _emitterrotation_4 _emitterscale_4)
          ;;;[0 0.5355 1] After hiding the bone, spawn the fake limb actor (that's falling down to the floor) using the SpawnDismemberedActor event.
          (CallFunction|SpawnDismemberedActor (.LeftArmMesh (Utilities|Struct|BreakS_LimbActors (Variables|DismembermentSetup|GetLimbActorsToSpawn))) (Math|Transform|MakeTransform _returnvalue_3 (Math|Rotator|MakeRotator 0.0 0.0 (.Yaw (Math|Rotator|BreakRotator (Transformation|GetSocketRotation (Variables|Default|GetOwnerMesh) _leftupperarmbone))))))
          ;;;[0 0.5355 1] Then spawn the attached emitter (to fake continous bleeding from the source) to the bone that's been hidden.
          (Effects|SpawnEmitterAttached (Variables|DismembermentEmitterSetup|GetLimbAttachedEmitter) (Variables|Default|GetOwnerMesh) (.LeftUpperArmSocketName (Utilities|Struct|BreakS_LimbSocketNames (Variables|DismembermentSetup|GetLimbSocketNames))) "0, 0, 0" (.LeftArmEmitterRotation (Utilities|Struct|BreakS_DismemberedEmitterRotations (Variables|DismembermentEmitterSetup|GetAttachedEmitterRotations)))))
        (elif (== _rightlegindex _dismemberedlimbindex)
          ;;[0 0.1294 0.2431] Right Leg Dismemberment Logic
          ;;;[0 0.5355 1] Check if the bone is hidden already (it's already dismembered)
          (bind _returnvalue_9 (Class|SkinnedMeshComponent|IsBoneHiddenbyName (Variables|Default|GetOwnerMesh) _rightthighbone))
          (if (not _returnvalue_9)
            ;;;[0 0.5355 1] If it's not dismembered, then dismember it by hiding the selected bone, and spawning the selected ReactionEmitter.
            (Components|SkinnedMesh|HideBonebyName _ownermesh_5 _rightthighbone "PBO_None")
            (CallFunction|ServerSpawnEmitteratLocation _emittertoplay_5 _returnvalue_4 _emitterrotation_5 _emitterscale_5)
            ;;;[0 0.5355 1] After hiding the bone, spawn the fake limb actor (that's falling down to the floor) using the SpawnDismemberedActor event.
            (CallFunction|SpawnDismemberedActor (.RightLegMesh (Utilities|Struct|BreakS_LimbActors (Variables|DismembermentSetup|GetLimbActorsToSpawn))) (Math|Transform|MakeTransform _returnvalue_4 (Math|Rotator|MakeRotator 0.0 0.0 (.Yaw (Math|Rotator|BreakRotator (Transformation|GetSocketRotation (Variables|Default|GetOwnerMesh) _rightthighbone))))))
            ;;;[0 0.5355 1] Then spawn the attached emitter (to fake continous bleeding from the source) to the bone that's been hidden.
            (Effects|SpawnEmitterAttached (Variables|DismembermentEmitterSetup|GetLimbAttachedEmitter) (Variables|Default|GetOwnerMesh) (.RightThighSocketName (Utilities|Struct|BreakS_LimbSocketNames (Variables|DismembermentSetup|GetLimbSocketNames))) "0, 0, 0" (.RightLegEmitterRotation (Utilities|Struct|BreakS_DismemberedEmitterRotations (Variables|DismembermentEmitterSetup|GetAttachedEmitterRotations)))))
          (elif (== _leftlegindex _dismemberedlimbindex)
            ;;[0 0.1294 0.2431] Right Leg Dismemberment Logic
            ;;;[0 0.5355 1] Check if the bone is hidden already (it's already dismembered)
            (bind _returnvalue_10 (Class|SkinnedMeshComponent|IsBoneHiddenbyName (Variables|Default|GetOwnerMesh) _leftthighbone))
            (if (not _returnvalue_10)
              ;;;[0 0.5355 1] If it's not dismembered, then dismember it by hiding the selected bone, and spawning the selected ReactionEmitter.
              (Components|SkinnedMesh|HideBonebyName _ownermesh_3 _leftthighbone "PBO_None")
              (CallFunction|ServerSpawnEmitteratLocation _emittertoplay _returnvalue_5 _emitterrotation _emitterscale)
              ;;;[0 0.5355 1] After hiding the bone, spawn the fake limb actor (that's falling down to the floor) using the SpawnDismemberedActor event.
              (CallFunction|SpawnDismemberedActor (.RightLegMesh (Utilities|Struct|BreakS_LimbActors (Variables|DismembermentSetup|GetLimbActorsToSpawn))) (Math|Transform|MakeTransform _returnvalue_5 (Math|Rotator|MakeRotator 0.0 0.0 (.Yaw (Math|Rotator|BreakRotator (Transformation|GetSocketRotation (Variables|Default|GetOwnerMesh) _leftthighbone))))))
              ;;;[0 0.5355 1] Then spawn the attached emitter (to fake continous bleeding from the source) to the bone that's been hidden.
              (Effects|SpawnEmitterAttached (Variables|DismembermentEmitterSetup|GetLimbAttachedEmitter) (Variables|Default|GetOwnerMesh) (.LeftThighSocketName (Utilities|Struct|BreakS_LimbSocketNames (Variables|DismembermentSetup|GetLimbSocketNames))) "0, 0, 0" (.LeftLegEmitterRotation (Utilities|Struct|BreakS_DismemberedEmitterRotations (Variables|DismembermentEmitterSetup|GetAttachedEmitterRotations)))))))))))

(event Custom|Multicast%20IncrementHitCounterOnLimb
  (params (LimbIndex :type Integer))
  (bind _returnvalue (Game|GetPlayerCharacter 0))
  (bind _returnvalue_2 (Components|GetOwner))
  (bind _limbhitcounterarray (Variables|Don'tTouch|GetLimbHitCounterArray))
  (bind _output (Utilities|Array|Get(acopy) _limbhitcounterarray LimbIndex))
  ;[1 1 1] Reaction - Called when owner's Event AnyDamage is played
  ;;[0 0.5355 1] Multicast IncrementHitCounterOnLimb - implements the HitCounterArray on the selected limb index, then checks if hits = required hits, if it is, call the HideDismemberedBone event, then kill the owner, or use a custom reaction.
  (Utilities|Array|SetArrayElem (Variables|Don'tTouch|GetLimbHitCounterArray) LimbIndex (+ _output 1))
  (bind _dismembered_ (CallFunction|CheckHitsonLimb))
  (if _dismembered_
    (CallFunction|ServerStartLimbDismemberment)
    (Class|BPIDeveloperOptions|UpdateHitsonLimb(Message) _returnvalue _output)
    (Utilities|FlowControl|Sequence
      (:then_0
        (if (Variables|DismembermentSetup|GetShouldKillOnAnyDismemberment?)
          (Class|BPIReactionComponent|InstantKillOwner(Message) _returnvalue_2)))
      (:then_1
        (if (Variables|CustomReactionsSetup|GetCustomReactionsOnDismemberment?)
          (Class|BPIReactionComponent|OwnerLimbDismembered(Message) _returnvalue_2 LimbIndex))))
    (else
      (Class|BPIDeveloperOptions|UpdateHitsonLimb(Message) _returnvalue _output))))

(event Custom|SpawnDismemberedActor
  (params (Class :type Actor%20Class%20Reference) (SpawnTransform :type Transform))
  ;[1 1 1] Spawning the Pseudo Limb Actors
  ;;[0 0.5355 1] Spawn DismemberedActor - Replicated to server - spawn the selected actor (the input Class of event, feeded in from Multicast Start Limb Dismemberment) and apply impulse to it. LimbActors need to be child actors of BP_LimbActor_Master to be able to receive impulse!
  (bind _returnvalue (Game|SpawnActorfromClass Class SpawnTransform "Undefined" 0 0))
  (bind _asbp_limb_actor_master (Utilities|Casting|CastToBP_LimbActor_Master _returnvalue))
  (CallFunction|MulticastAddImpulsetoDismemberedLimb (Variables|/Game/ReactionSystemBP/DemoContent/Blueprints/Limbs/BP_LimbActor_Master.BP_LimbActor_Master_C|GetMesh _asbp_limb_actor_master) (* (* (Transformation|GetActorForwardVector (Components|GetOwner)) (Variables|DismembermentSetup|GetDismembermentImpulseForce)) -1.0)))

(event Custom|Multicast%20Spawn%20Emitter%20At%20Location
  (params (Emitter%20To%20Spawn :type Particle%20System%20Object%20Reference) (Location :type Vector) (Rotation :type Rotator) (Scale :type Vector))
  ;[1 1 1] Effects - From HideDismemberedBone event
  ;;[0 0.5355 1] Spawn Emitter At Location replicated
  (Effects|SpawnEmitteratLocation Emitter%20To%20Spawn Location Rotation Scale))

(event Custom|Server%20Spawn%20Emitter%20At%20Location
  (params (Emitter%20To%20Spawn :type Particle%20System%20Object%20Reference) (Location :type Vector) (Rotation :type Rotator) (Scale :type Vector))
  ;[1 1 1] Effects - From HideDismemberedBone event
  ;;[0 0.5355 1] Spawn Emitter At Location replicated
  (bind _output_get (Variables|Don'tTouch|SetSpawnedEmitter Emitter%20To%20Spawn))
  (CallFunction|MulticastSpawnEmitteratLocation _output_get Location Rotation Scale))

(event Custom|Multicast%20Add%20Impulse%20To%20Dismembered%20Limb
  (params (Target :type Primitive%20Component%20Object%20Reference) (Impulse :type Vector))
  ;[1 1 1] Spawning the Pseudo Limb Actors
  ;;[0 0.5355 1] Multicast Add ImpulseToDismemberedLimb - a multicast replicated impulse (to make sure the clients and server receive the same impulse amount)
  (Physics|AddImpulse Target Impulse "None" true))

(event Custom|IncrementHitCounterOnLimb
  (params (LimbIndex :type Integer))
  ;[1 1 1] Reaction - Called when owner's Event AnyDamage is played
  ;;[0 0.5355 1] IncrementHitCounterOnLimb - check if dismemberment is enabled.
  (if (Variables|DismembermentSetup|GetShouldUseLimbDismemberment?)
    (CallFunction|MulticastIncrementHitCounteronLimb LimbIndex)))

(event Custom|Server%20Start%20Limb%20Dismemberment
  ;[1 1 1] Start Limb Dismemberment - The main event of the dismemberment component - hides dismembered bone, spawns emitters, spawn fake limb
  ;;[0 0.5355 1] Called from MulticastIncrementHitCounterOnLimb
  (CallFunction|MulticastStartLimbDismemberment))

(event EventBeginPlay
  ;[1 1 1] Initialization - When owner actor is spawned
  ;;[0 0.5355 1] Beginplay - Set the "OwnerMesh" ref to use when modifying the owner's skeletal mesh.
  (bind _mesh (Class|BPIReactionComponent|GetOwnerMesh(Message) (Components|GetOwner)))
  (Variables|Default|SetOwnerMesh _mesh))

(fn SetCurrentLimbIndex
  (params (TracedBone :type Name))
  (bind _bonenamestructure (Variables|DismembermentSetup|GetBoneNameStructure))
  (bind _bonenamestructure_2 (Variables|DismembermentSetup|GetBoneNameStructure))
  (bind _bonenamestructure_3 (Variables|DismembermentSetup|GetBoneNameStructure))
  (bind _bonenamestructure_4 (Variables|DismembermentSetup|GetBoneNameStructure))
  (bind (_hipbone _headbone _leftthighbone _leftcalfbone _leftfootbone _rightthighbone _rightcalfbone _rightfootbone _spine_01bone _spine_02bone _spine_03bone _leftclaviclebone _leftupperarmbone _leftlowerarmbone _rightclaviclebone _rightupperarmbone _rightlowerarmbone) (Utilities|Struct|BreakS_BoneNames _bonenamestructure))
  (bind (_hipbone_2 _headbone_2 _leftthighbone_2 _leftcalfbone_2 _leftfootbone_2) (Utilities|Struct|BreakS_BoneNames _bonenamestructure_3))
  (bind (_hipbone_3 _headbone_3 _leftthighbone_3 _leftcalfbone_3 _leftfootbone_3 _rightthighbone_2 _rightcalfbone_2 _rightfootbone_2) (Utilities|Struct|BreakS_BoneNames _bonenamestructure_4))
  (bind (_hipbone_4 _headbone_4 _leftthighbone_4 _leftcalfbone_4 _leftfootbone_4 _rightthighbone_3 _rightcalfbone_3 _rightfootbone_3 _spine_01bone_2 _spine_02bone_2 _spine_03bone_2 _leftclaviclebone_2 _leftupperarmbone_2 _leftlowerarmbone_2) (Utilities|Struct|BreakS_BoneNames _bonenamestructure_2))
  ;[1 1 1] Set Current Limb Index - From Event AnyDamage on owner characters.
  ;;[0 0.5355 1] Saving the inputted tracedBone as a local variable so it can be used many times during the function without the unnecesary wires.
  (LocalVariables|SetLocalTracedBoneName TracedBone)
  ;;[0 0.5355 1] Select if the Traced bone is the headbone
  (if (Utilities|Name|Equal(Name) (LocalVariables|GetLocalTracedBoneName) (.HeadBone (Utilities|Struct|BreakS_BoneNames (Variables|DismembermentSetup|GetBoneNameStructure))))
    ;;[0 0.5355 1] Set The CurrentLimbIndex's value to the HeadIndex (That's been set up in the LimbArrayIndex)
    (bind _output_get (Variables|Don'tTouch|SetCurrentLimbIndex (.HeadIndex (Utilities|Struct|BreakS_LimbArrayIndex (Variables|DismembermentSetup|GetLimbArrayIndex)))))
    (return true _output_get)
    (else
      ;;[0 0.5355 1] Select if the Traced bone is the one of the Leftleg bones (Thigh,Calf,Foot)
      (if (Math|Boolean|ORBoolean (Utilities|Name|Equal(Name) (LocalVariables|GetLocalTracedBoneName) _leftthighbone_2) (Utilities|Name|Equal(Name) (LocalVariables|GetLocalTracedBoneName) _leftcalfbone_2) (Utilities|Name|Equal(Name) (LocalVariables|GetLocalTracedBoneName) _leftfootbone_2))
        ;;[0 0.5355 1] Set CurrentLimbIndex to the LeftLegIndex
        (bind _output_get_2 (Variables|Don'tTouch|SetCurrentLimbIndex (.LeftLegIndex (Utilities|Struct|BreakS_LimbArrayIndex (Variables|DismembermentSetup|GetLimbArrayIndex)))))
        (return true _output_get_2)
        (else
          ;;[0 0.5355 1] Select if the TracedBone is one of the RightLeg bones (Thigh,Calf,Foot)
          (if (Math|Boolean|ORBoolean (Utilities|Name|Equal(Name) (LocalVariables|GetLocalTracedBoneName) _rightthighbone_2) (Utilities|Name|Equal(Name) (LocalVariables|GetLocalTracedBoneName) _rightcalfbone_2) (Utilities|Name|Equal(Name) (LocalVariables|GetLocalTracedBoneName) _rightfootbone_2))
            ;;[0 0.5355 1] Set CurrentLimbIndex to the RightLegIndex
            (bind _output_get_3 (Variables|Don'tTouch|SetCurrentLimbIndex (.RightLegIndex (Utilities|Struct|BreakS_LimbArrayIndex (Variables|DismembermentSetup|GetLimbArrayIndex)))))
            (return true _output_get_3)
            (else
              ;;[0 0.5355 1] Select if the TracedBone is one of the LeftArm bones (Clavicle,Upper,LowerArm)
              (if (Math|Boolean|ORBoolean (Utilities|Name|Equal(Name) (LocalVariables|GetLocalTracedBoneName) _leftclaviclebone_2) (Utilities|Name|Equal(Name) (LocalVariables|GetLocalTracedBoneName) _leftupperarmbone_2) (Utilities|Name|Equal(Name) (LocalVariables|GetLocalTracedBoneName) _leftlowerarmbone_2))
                ;;[0 0.5355 1] Set CurrentLimbIndex to the LeftArmIndex
                (bind _output_get_4 (Variables|Don'tTouch|SetCurrentLimbIndex (.LeftArmIndex (Utilities|Struct|BreakS_LimbArrayIndex (Variables|DismembermentSetup|GetLimbArrayIndex)))))
                (return true _output_get_4)
                (else
                  ;;[0 0.5355 1] Select if the TracedBone is one of the RightArm bones (Clavicle,Upper,LowerArm)
                  (if (Math|Boolean|ORBoolean (Utilities|Name|Equal(Name) (LocalVariables|GetLocalTracedBoneName) _rightclaviclebone) (Utilities|Name|Equal(Name) (LocalVariables|GetLocalTracedBoneName) _rightupperarmbone) (Utilities|Name|Equal(Name) (LocalVariables|GetLocalTracedBoneName) _rightlowerarmbone))
                    ;;[0 0.5355 1] Set CurrentLimbIndex to the RightArmIndex
                    (bind _output_get_5 (Variables|Don'tTouch|SetCurrentLimbIndex (.RightArmIndex (Utilities|Struct|BreakS_LimbArrayIndex (Variables|DismembermentSetup|GetLimbArrayIndex)))))
                    (return true _output_get_5)
                    (else
                      ;;[0 0.5355 1] If the TracedBone is none of the previous bones, return the function as Unssuccesful.
                      (return false 0))))))))))))

(fn CheckHitsonLimb
  ;[1 1 1] Check Hits on selected Limb
  ;;[0 0.5355 1] Check if the hits on the selected limb (CurrentLimbIndex ) are >= the required amount.
  (if (>= (Utilities|Array|Get(acopy) (Variables|Don'tTouch|GetLimbHitCounterArray) (Variables|Don'tTouch|GetCurrentLimbIndex)) (Variables|DismembermentSetup|GetHitsRequiredForDismemberment))
    ;;[0 0.5355 1] If the hits are enough on the limb, check if the limb is dismemberable
    (if (Utilities|Array|Get(acopy) (Variables|DismembermentSetup|GetDismemberableLimbs) (Variables|Don'tTouch|GetCurrentLimbIndex))
      ;;[0 0.5355 1] if the limb is dismemberable, set the "DismemberedLimbIndex" to the current limb index (it's used in MulticastHideDismemberedBone" event) then set the "DismemberedLimbs" bool array's value at the index to true.
      (bind _output_get (Variables|Don'tTouch|SetDismemberedLimbIndex (Variables|Don'tTouch|GetCurrentLimbIndex)))
      (Utilities|Array|SetArrayElem (Variables|Don'tTouch|GetDismemberedLimbs) _output_get true)
      (return true)
      (else
        ;;[0 0.5355 1] If it's not, return false.
        (return false)))
    (else
      ;;[0 0.5355 1] If the hits are not enough, return false
      (return false))))

(fn CheckLimbDismembered
  (params (Limb%20Index :type Integer))
  (if (Utilities|Array|Get(acopy) (Variables|Don'tTouch|GetDismemberedLimbs) Limb%20Index)
    (return true)
    (else
      (return false))))