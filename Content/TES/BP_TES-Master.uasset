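; BP_TES-Master is the player's interaction system, detecting interactable objects and forwarding input to them.
; Looping timers sphere-trace from the camera for the focused actor, and overlap around the pawn to show widgets on nearby actors in line of sight.
; E sends an interface message to the focused actor, while alternate-interact and shot events use a separate line trace to call BP_MasterActor.
; HoldTrace suspends detection; EquipWeapon is an empty stub.
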(event Custom|InteractHitActor
  (Class|BPInteractionInterface|Interaction(Message) (Variables|Interaction|GetFocusedActor) 0 "NewEnumerator0"))

(event Custom|AlternativeInteractHitActor
  (bind _hit_actor (Utilities|GetInteractable)
    (:%20%20%20%20
      (bind _asbp_master_actor (Utilities|Casting|CastToBP_MasterActor _hit_actor))
      (if (Variables|/Game/TES/BP_MasterActor.BP_MasterActor_C|GetinteractionEnabled? _asbp_master_actor)
        (Default|AltInteract _asbp_master_actor)))))

(event Custom|ShotHitActor
  (bind _hit_actor (Utilities|GetInteractable)
    (:%20%20%20%20
      (bind _asbp_master_actor (Utilities|Casting|CastToBP_MasterActor _hit_actor))
      (if (Variables|/Game/TES/BP_MasterActor.BP_MasterActor_C|GetinteractionEnabled? _asbp_master_actor)
        (Default|Shot _asbp_master_actor)))))

(event Custom|EquipWeapon
  (params (EquipType :type E_EquipType%20Enum :default "NewEnumerator3")))

(event EventBeginPlay
  ;[1 0.1448 0.9419] Begin Setup
  (bind _returnvalue (Game|GetCurrentLevelName true))
  (CallFunction|PlayerInput (not (Utilities|Enum|Equal(Enum) _returnvalue "MenuLevel")))
  (Utilities|Time|SetTimerbyFunctionName 0 "TraceForInteraction" 0.1 true)
  (Utilities|Time|SetTimerbyFunctionName 0 "FindAndHighlightObjectsNearPlayer" 0.1 true))

(event Input|KeyboardEvents|E
  (params (Key :type Key%20Structure))
  (:Pressed
    (CallFunction|InteractHitActor)))

(fn ConstructionScript)

(fn TraceforInteraction
  (bind _returnvalue (Game|GetPlayerCameraManager 0))
  (bind _returnvalue_2 (Camera|GetCameraLocation _returnvalue))
  (if (not (Variables|Interaction|GetHoldTrace))
    (bind _outhit (Collision|SphereTraceForObjects _returnvalue_2 (+ _returnvalue_2 (* (Transformation|GetActorForwardVector _returnvalue) (Variables|Interaction|GetInteractDistance)) (* (Transformation|GetActorUpVector _returnvalue) 3e+01) (* (Transformation|GetActorRightVector _returnvalue) -3e+01)) 3e+01 (Utilities|Array|MakeArray "ObjectTypeQuery7" "ObjectTypeQuery1" "ObjectTypeQuery2") false (Utilities|Array|MakeArray (Game|Player|GetPlayerPawn 0)) "None" true "(R=1.000000,G=0.000000,B=0.000000,A=1.000000)" "(R=0.000000,G=1.000000,B=0.000000,A=1.000000)" 2.0))
    (if (.bblockinghit _outhit)
      (if (Utilities|Enum|Equal(Enum) (Collision|GetCollisionObjectType (.hitcomponent _outhit)) "ECC_GameTraceChannel1")
        (Variables|Interaction|SetFocusedActor (.hitactor _outhit))
        (Variables|Default|SetFocusedComponent (.hitcomponent _outhit))
        (Class|BPInteractionInterface|ButtonWidgetVisibility(Message) (Variables|Interaction|GetFocusedActor) true false)
        (else
          (bind _focusedactor (Variables|Interaction|GetFocusedActor :!label _label)
            (:then
              (Class|BPInteractionInterface|ButtonWidgetVisibility(Message) _focusedactor false false))
            (:else
              _))
          (Variables|Interaction|SetFocusedActor 0)
          (Variables|Default|SetFocusedComponent 0)))
      (else
        (goto _label)))))

(fn FindandHighlightObjectsNearPlayer
  (bind _returnvalue (Game|Player|GetPlayerPawn 0))
  (if (Variables|Interaction|GetHoldTrace)
    (for _array_element (Variables|Default|GetCloseActors)
      (bind _enabled (Class|BPInteractionInterface|IsEnabled?(Message) _array_element))
      (if _enabled
        (Class|BPInteractionInterface|ButtonWidgetVisibility(Message) _array_element false false)
        (Utilities|Array|RemoveItem (Variables|Default|GetCloseActors) _array_element)
        (Class|BPInteractionInterface|ToggleObjectOutline(Message) _array_element false)))
    (else
      (bind _outactors (Collision|SphereOverlapActors (Transformation|GetActorLocation _returnvalue) (Variables|Default|GetObjectDisplayDistance) (Utilities|Array|MakeArray "ObjectTypeQuery7") 0 (Utilities|Array|MakeArray _returnvalue)))
      (bind _output_get (Variables|Default|SetCloseActors _outactors))
      (for _array_element_2 _output_get
        (|IsActorVisibleForPlayer? _array_element_2
          (:Is%20Visible
            (if (!= (Variables|Interaction|GetFocusedActor) _array_element_2)
              (bind _enabled_2 (Class|BPInteractionInterface|IsEnabled?(Message) _array_element_2))
              (if _enabled_2
                (Class|BPInteractionInterface|ButtonWidgetVisibility(Message) _array_element_2 true true)
                (Utilities|Time|SetTimerbyFunctionName _array_element_2 "CheckIfWidgetShouldBeVisible" 0.1 true)))))))))