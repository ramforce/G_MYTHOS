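; Save-game component that snapshots player state and BP_MasterActor TES events into a PlayerSaveGame in slot "test".
; Collect functions fill caches that SaveVariables writes with level name and date; RestorePlayer reapplies transform, objective, weapon, points, health and ability.
; EventGraph save, load and restore chains are disconnected from their empty events, so none run.
; Environment and ambient collectors are empty, and LoadVariables is unwired.
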(event Custom|SaveGame)

(event Custom|LoadGame
  (params (NewParam :type String)))

(event Custom|LoadLastSave)

(event Custom|BeginEvent
  (params (Player :type Actor%20Object%20Reference)))

(event EventBeginPlay)

(event EventTick
  (params (DeltaSeconds :type Float%20%28single-precision%29)))

(fn GetDate
  (bind _returnvalue (Math|DateTime|Now))
  (bind (_year _month _day _hour _minute _second) (Math|DateTime|BreakDateTime _returnvalue))
  (return (Utilities|Text|ToText(String) (Utilities|String|Append (Utilities|String|ToString(Integer) _year) "." (Utilities|String|ToString(Integer) _month) "." (Utilities|String|ToString(Integer) _day) " " (Utilities|String|ToString(Integer) _hour) ":" (Utilities|String|ToString(Integer) _minute) ":" (Utilities|String|ToString(Integer) _second)))))