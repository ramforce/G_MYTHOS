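; BP_MasterPickup is a TES pickup Blueprint that responds to interaction and being shot through the TES event system.
; Its construction script passes the CreateTESEvent data to TMDefaultConstructions.
; At BeginPlay it casts itself to BP_MasterActor and copies that data into TESEvents.
; Interact and Shot each call TESEventCheck with their own enum value.
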(event EventBeginPlay
  (bind _asbp_master_actor (Utilities|Casting|CastToBP_MasterActor self))
  (Variables|/Game/TES/BP_MasterActor.BP_MasterActor_C|SetTES%20Events _asbp_master_actor (Variables|Default|GetCreate%20TES%20Event)))

(event EventShot
  (CallFunction|TESEventCheck "NewEnumerator11"))

(event EventInteract
  (CallFunction|TESEventCheck "NewEnumerator1"))

(fn ConstructionScript
  (Utilities|TMDefaultConstructions (Variables|Default|GetCreate%20TES%20Event)))