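; Base actor for the TES event system, with empty stubs for interaction and state actions such as open/close, lock, flicker, alarm and shot.
; TESEventCheck increments counters on TESEvents entries matching the given trigger interaction and caches those reaching their AfterNTimes threshold, with separate do-once and counter-reset branches.
; It then spawns a TESEvent actor per cached entry, passes it that event's data and clears the cache.
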(event EventBeginPlay)

(event Collision|EventActorBeginOverlap
  (params (OtherActor :type Actor%20Object%20Reference)))

(event EventTick
  (params (DeltaSeconds :type Float%20%28single-precision%29)))

(fn ConstructionScript)

(fn Interact)

(fn AltInteract)

(fn TESEventCheck
  (params (Check :type E_TriggerTypes%20Enum :default "NewEnumerator0"))
  (bind _tes_events (Variables|Default|GetTES%20Events))
  (bind _indexcache (Variables|Default|GetIndexCache))
  (for (_array_element _array_index) _tes_events
    (if (Utilities|Enum|Equal(Enum) (.TriggerInteraction (Utilities|Struct|BreakTES_EventMaster _array_element)) Check)
      (bind _structout (Utilities|Struct|SetmembersinTES_EventMaster _array_element (+ (.Counter (Utilities|Struct|BreakTES_EventMaster _array_element)) 1)))
      (Utilities|Array|SetArrayElem _tes_events _array_index _structout)
      (if (== (.AfterNTimes (Utilities|Struct|BreakTES_EventMaster _array_element)) (.Counter (Utilities|Struct|BreakTES_EventMaster _array_element)))
        (Utilities|Array|Add (Variables|Default|GetIndexCache) _array_index)
        (if (.DoOnce (Utilities|Struct|BreakTES_EventMaster _array_element))
          (bind _structout_2 (Utilities|Struct|SetmembersinTES_EventMaster _array_element))
          (Utilities|Array|SetArrayElem _tes_events _array_index _structout_2)
          (else
            ;[0 0.1099 1] Do (N) Times
            (bind _structout_3 (Utilities|Struct|SetmembersinTES_EventMaster _array_element))
            (Utilities|Array|SetArrayElem _tes_events _array_index _structout_3))))))
  (for _array_element_2 _indexcache
    (bind _returnvalue (Game|SpawnActorfromClass "/Game/TES/TES-Event.TES-Event_C" (Math|Transform|MakeTransform "0, 0, 0" "0, 0, 0" "1,1,1") "Undefined" 0 0))
    (Default|TESEvent _returnvalue (Utilities|Struct|BreakTES_EventMaster (Utilities|Array|Get(acopy) (Variables|Default|GetTES%20Events) _array_element_2))))
  (Utilities|Array|Clear _indexcache))

(fn Open/On)

(fn Close/Off)

(fn Lock)

(fn Unlock)

(fn Flicker)

(fn Unflicker)

(fn Alarm)

(fn Disalarm)

(fn Shot)