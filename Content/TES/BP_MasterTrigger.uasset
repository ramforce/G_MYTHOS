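; BP_MasterTrigger is a trigger actor that runs a TES event check when the player pawn overlaps it.
; The construction script passes CreateTESEvent to TMDefaultConstructions.
; On BeginPlay it casts itself to BP_MasterTrigger and copies CreateTESEvent into TESEvents.
; Overlaps by the first player's pawn call TESEventCheck with a fixed enum value, and other actors are ignored.
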(event EventBeginPlay
  (bind _asbp_master_trigger (Utilities|Casting|CastToBP_MasterTrigger self))
  (Variables|/Game/TES/BP_MasterActor.BP_MasterActor_C|SetTES%20Events _asbp_master_trigger (Variables|Default|GetCreate%20TES%20Event)))

(event Collision|EventActorBeginOverlap
  (params (OtherActor :type Actor%20Object%20Reference))
  (if (== OtherActor (Game|Player|GetPlayerPawn 0))
    (CallFunction|TESEventCheck "NewEnumerator2")))

(fn ConstructionScript
  (Utilities|TMDefaultConstructions (Variables|Default|GetCreate%20TES%20Event)))