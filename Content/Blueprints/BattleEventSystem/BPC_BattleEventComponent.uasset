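; Battle event component on each unit that tracks nearby and sighted units and fires the character's quirks in response.
; BeginPlay caches trigger types from the quirks data table.
; Range, movement, environment and surrounding events call shared BE functions to update range and sight, handle internal quirks, and refresh a debug HUD.
; External-unit quirk handling is an empty event, with its loop and the lost-sight branch left disconnected.
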(event Custom|HandleInternalQuirks
  (params (Quirk%20Trigger :type E_QuirkTriggerType%20Enum :default "NewEnumerator0") (Instigator%20BPC :type BPC%20Battle%20Event%20Component%20Object%20Reference))
  (CallFunction|BEHandleQuirks self Instigator%20BPC Quirk%20Trigger))

(event Custom|SurroundingUpdate
  (params (New%20Surrounding :type E_SurroundingType%20Enum :default "NewEnumerator3"))
  (Variables|Environment|SetCurrentSurrounding New%20Surrounding)
  (CallFunction|HandleInternalQuirks "NewEnumerator0" self))

(event Custom|EnvironmentUpdate
  (params (New%20Environment :type E_EnvironmentType%20Enum :default "NewEnumerator7"))
  (Variables|Environment|SetCurrentEnvironment New%20Environment)
  (CallFunction|HandleInternalQuirks "NewEnumerator0" self))

(event Custom|ActorInRangeCheck
  (params (Actor%20In :type Actor%20Object%20Reference) (Owner%20Actor :type Actor%20Object%20Reference))
  (bind _debughud (Variables|Setup|GetDebugHUD))
  ;[1 0 0.1875] Triggered on each Unit
  ;;[0.5 1 0] Check if Actor is in Close Range
  (Variables|Environment|SetisPerformingRangeCheck true)
  (CallFunction|BEActorinRange Actor%20In Owner%20Actor (Variables|Setup|GetDrawDebug?))
  (bind _unit_ids (CallFunction|GetNearbyUnitIDs (Variables|Environment|GetUnitsInCloseRange)))
  (Default|UpdateActorsinRange _debughud _unit_ids)
  (bind _unit_ids_2 (CallFunction|GetNearbyUnitIDs (Variables|Environment|GetUnitsInCloseSight)))
  (Default|UpdateActorsinSight _debughud _unit_ids_2)
  (Variables|Environment|SetisPerformingRangeCheck false))

(event Custom|UpdateActorInRangeOnMove
  ;[0 1 0.4141] Update Actor in Sight on Movement - Triggered on possessed Unit only
  (if (> (Utilities|Array|Length (Variables|Environment|GetUnitsInCloseRange)) 0)
    (for _array_element (Variables|Environment|GetUnitsInCloseRange)
      (Utilities|IsValid (Actor|GetComponentbyClass _array_element "BPC_BattleEventComponent_C")
        (:Is%20Valid
          (bind _insight_ (CallFunction|BEActorinSight self (Actor|GetComponentbyClass _array_element "BPC_BattleEventComponent_C") (Variables|Setup|GetDrawDebug?))))))
    (bind _unit_ids (CallFunction|GetNearbyUnitIDs (Variables|Environment|GetUnitsInCloseSight)))
    (Default|UpdateActorsinSight (Variables|Setup|GetDebugHUD) _unit_ids)
    (CallFunction|HandleQuirksforExternalUnits (Variables|Environment|GetUnitsInCloseSight) "NewEnumerator8")))

(event Custom|ActorLeftRange
  (params (Actor%20In :type Actor%20Object%20Reference) (Owner%20Actor :type Actor%20Object%20Reference))
  (bind _returnvalue (Actor|GetComponentbyClass Actor%20In "BPC_BattleEventComponent_C"))
  (bind _returnvalue_2 (Actor|GetComponentbyClass Owner%20Actor "BPC_BattleEventComponent_C"))
  (bind _debughud (Variables|Setup|GetDebugHUD))
  ;[1 0 0.1875] Triggered on each Unit
  ;;[1 0.375 0] Actor No Longer in Close Range
  (Utilities|IsValid _returnvalue
    (:Is%20Valid
      (Variables|Environment|SetisPerformingRangeCheck true)
      (CallFunction|BEActorLeftRange _returnvalue _returnvalue_2)
      (CallFunction|HandleInternalQuirks _returnvalue_2 "NewEnumerator8" _returnvalue)
      (bind _unit_ids (CallFunction|GetNearbyUnitIDs (Variables|Environment|GetUnitsInCloseSight)))
      (Default|UpdateActorsinSight _debughud _unit_ids)
      (bind _unit_ids_2 (CallFunction|GetNearbyUnitIDs (Variables|Environment|GetUnitsInCloseRange)))
      (Default|UpdateActorsinRange _debughud _unit_ids_2)
      (Variables|Environment|SetisPerformingRangeCheck false))))

(event Custom|HandleQuirksForExternalUnits
  (params (Target%20Units :type Array%20of%20Actor%20Object%20References) (Quirk%20Trigger :type E_QuirkTriggerType%20Enum :default "NewEnumerator0")))

(event EventBeginPlay
  (bind _quirktriggerarray (Variables|Quirks|GetQuirkTriggerArray))
  ;[1 0.08091 0.3539] Quirk Trigger Array
  (Utilities|Array|Clear _quirktriggerarray)
  (for _array_element (Utilities|Struct|BreakCharacter_Struct (Variables|Setup|GetCharacterInfo))
    (bind _returnvalue (Utilities|GetDataTableRow "/Game/Blueprints/Data/Quirks/Quirks_DataTable.Quirks_DataTable" _array_element)
      (:then
        (Utilities|Array|AddUnique _quirktriggerarray (Utilities|Struct|BreakQuirks_Struct _returnvalue))))))

(fn GetNearbyUnitIDs
  (params (Unit%20Actors :type Array%20of%20Actor%20Object%20References))
  (bind _unitnames (LocalVariables|GetUnitNames))
  (for _array_element Unit%20Actors
    (Utilities|IsValid (Actor|GetComponentbyClass _array_element "BPC_BattleEventComponent_C")
      (:Is%20Valid
        (Utilities|Array|AddUnique _unitnames (.name (Variables|BPC_BattleEventComponent_C|GetCharacterInfo (Actor|GetComponentbyClass _array_element "BPC_BattleEventComponent_C")))))))
  (return _unitnames))