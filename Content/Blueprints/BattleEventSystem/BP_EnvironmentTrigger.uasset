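; BP_EnvironmentTrigger is a trigger volume that sets the environment and surrounding state of actors entering it, as part of the battle event system.
; On box begin overlap, it ignores components tagged RangeCheckOnly and passes both enums to the actor's BPC_BattleEventComponent.
; Each enum has one value that skips its update, and nothing runs on exit.
; The construction script labels the volume with either enum's name via a debug toggle.
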(event OnComponentBeginOverlap(Box)
  (params (OverlappedComponent :type Primitive%20Component%20Object%20Reference) (OtherActor :type Actor%20Object%20Reference) (OtherComp :type Primitive%20Component%20Object%20Reference) (OtherBodyIndex :type Integer) (bFromSweep :type Boolean) (SweepResult :type Hit%20Result%20Structure%20%28by%20ref%29))
  (bind _returnvalue (Actor|GetComponentbyClass OtherActor "/Game/Blueprints/BattleEventSystem/BPC_BattleEventComponent.BPC_BattleEventComponent_C"))
  (bind _environment (Variables|Default|GetEnvironment))
  (bind _surrounding (Variables|Default|GetSurrounding))
  (if (not (Utilities|Array|ContainsItem (Variables|/Script/Engine.ActorComponent|GetComponentTags OtherComp) "RangeCheckOnly"))
    (Utilities|IsValid _returnvalue
      (:Is%20Valid
        (if (Utilities|Enum|NotEqual(Enum) _environment "NewEnumerator7")
          (Default|EnvironmentUpdate _returnvalue _environment))
        (if (Utilities|Enum|NotEqual(Enum) _surrounding "NewEnumerator3")
          (Default|SurroundingUpdate _returnvalue _surrounding))))))

(event EventBeginPlay)

(event Collision|EventActorBeginOverlap
  (params (OtherActor :type Actor%20Object%20Reference)))

(event EventTick
  (params (DeltaSeconds :type Float%20%28single-precision%29)))

(fn ConstructionScript
  (Rendering|Components|TextRender|SetText (Variables|Default|GetTextRender) (select (Variables|Default|GetDebugShowSurrounding) (Utilities|Text|ToText(String) (Utilities|String|EnumtoString (Variables|Default|GetSurrounding))) (Utilities|Text|ToText(String) (Utilities|String|EnumtoString (Variables|Default|GetEnvironment))))))