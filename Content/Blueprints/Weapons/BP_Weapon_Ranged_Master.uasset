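; Master ranged weapon Blueprint that loads its stats from a data table row and fires bullet projectiles.
; FireWeapon triggers camera shake, AI noise, pitch-varied and low-ammo sounds and muzzle flash.
; Bullets follow the laser sight's per-tick trace when active, otherwise a crosshair trace with movement-dependent spread applied to the look-at origin.
; Recoil and shot-delay nodes are disconnected, and ammo is only read, never decremented.
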(event Custom|CalculateProjectileRotation
  (params (WeaponMuzzleLocation :type Vector%20%28by%20ref%29) (LineTraceStart :type Vector) (LineTraceEnd :type Vector))
  (bind _returnvalue (CallFunction|CalculateAccuracy WeaponMuzzleLocation))
  ;[0 1 0.1797] Calculate Projectile Rotation - rotates the projectile to face the center of the screen
  ;;[0 0.5355 1] Spawn a line trace from the camera location towards the center of the screen.
  (bind _debuggingon_ (Class|BPIDeveloperOptions|IsDebuggingOn?(Message) (Components|GetOwner)))
  (bind (_outhit _returnvalue_2) (Collision|LineTraceByChannel LineTraceStart LineTraceEnd "TraceTypeQuery1" false (Utilities|Array|MakeArray (Components|GetOwner) self (Game|GetPlayerCharacter 0)) (select _debuggingon_ "ForDuration" "None")))
  ;;[0 0.5355 1] Check if there was a hit. (an actor blocks the visibility channel)
  (if _returnvalue_2
    ;;[0 0.5355 1] If there was, Find the rotation from the muzzle location (spawn point of bullet) towards the impact point (actor in the middle of the screen)
    (Variables|Don'tTouch|SetProjectileTowardsCrosshairRot (Math|Rotator|FindLookatRotation _returnvalue (.ImpactPoint (Collision|BreakHitResult _outhit))))
    (else
      ;;[0 0.5355 1] If there was not any hit, Find the rotation from the muzzle location (spawn point of bullet) towards the end of the line trace
      (Variables|Don'tTouch|SetProjectileTowardsCrosshairRot (Math|Rotator|FindLookatRotation _returnvalue (.TraceEnd (Collision|BreakHitResult _outhit)))))))

(event Custom|FireWeapon
  (bind _currentweaponinfo (Variables|Default|GetCurrentWeaponInfo))
  (bind _currentweaponinfo_2 (Variables|Default|GetCurrentWeaponInfo))
  (bind _muzzlearrow (Variables|Default|GetMuzzleArrow))
  (bind (_weaponname _weaponeffects _firerate _sounds _weaponshakeclass) (Utilities|Struct|BreakWeapon_Struct _currentweaponinfo))
  (bind (_weaponname_2 _weaponammo _weaponeffects_2 _burstlength _burstinterval _firerate_2 _automatic _holstersocket _equipsockets _weaponactionanim _weaponanimspeed _shotdecal _sounds_2) (Utilities|Struct|BreakWeapon_Struct _currentweaponinfo_2))
  (bind _returnvalue (Transformation|GetWorldLocation _muzzlearrow))
  (bind (_equipsound _shotsound _reloadsound _reloadwhenemptysound _lowammosound _verylowammosound _noammosound _loudness _firingpitchvariation _basepitch) (Utilities|Struct|BreakWeaponSound_Struct _sounds_2))
  (bind (_outputsound _outputpitch) (CallFunction|CalculateShotVolume _shotsound _firingpitchvariation _basepitch))
  ;[0 0.9766 1] FireWeapon
  ;;[1 0 0.2812] Camera Shake + Recoil
  (bind _asbp_mythos_character_master (Utilities|Casting|CastToBP_MythosCharacter_Master (Components|GetOwner)))
  (Variables|/Game/Blueprints/Core/BP_MythosCharacter_Master.BP_MythosCharacter_Master_C|SetisFiring? _asbp_mythos_character_master true)
  (Game|Feedback|ClientStartCameraShake (Game|GetPlayerController 0) _weaponshakeclass 1.0 "CameraLocal" "0, 0, 0")
  (Class|Pawn|PawnMakeNoise (Game|Player|GetPlayerPawn 0) (.Loudness (Utilities|Struct|BreakWeaponSound_Struct _sounds)) (Transformation|GetActorLocation) true 0)
  (if (not (< (.ClipAmmo (Utilities|Struct|BreakWeaponAmmo_Struct _weaponammo)) 1))
    (Audio|PlaySoundatLocation _outputsound (Transformation|GetWorldLocation (Variables|Default|GetMuzzleArrow)) "0, 0, 0" 1.0 _outputpitch 0.0 0 0 0)
    (|LowAmmoSFX
      (:%20
        (CallFunction|CalculateProjectileRotation _returnvalue (.Start (Default|CalculateFireTraceLoc _asbp_mythos_character_master)) (.End (Default|CalculateFireTraceLoc _asbp_mythos_character_master)))
        (bind _possessed_bpc (CallFunction|BEGetPossessedBPC))
        (Game|SpawnActorfromClass "/Game/Blueprints/Weapons/BP_Projectile_Bullet.BP_Projectile_Bullet_C" (Math|Transform|MakeTransform _returnvalue (select (Variables|Don'tTouch|GetIsLaserSightActive?) (Variables|Don'tTouch|GetLaserSightRotation) (Variables|Don'tTouch|GetProjectileTowardsCrosshairRot))) "Undefined" self (Variables|/Game/Blueprints/BattleEventSystem/BPC_BattleEventComponent.BPC_BattleEventComponent_C|GetOwningUnit _possessed_bpc))
        (Effects|SpawnEmitteratLocation "/Game/ReactionSystemBP/DemoContent/Effects/ParticleSystems/PS_Launcher_MuzzleFlash.PS_Launcher_MuzzleFlash" (Transformation|GetWorldLocation (Variables|Default|GetMuzzleArrow)) "0, 0, 0" "0.500000,0.500000,0.500000")))))

(event Custom|EmptyGunSFX
  ;[0 0.03906 1] Empty Gun SFX
  (Utilities|FlowControl|DoOnce false :!label _label
    (:Completed
      (Utilities|FlowControl|Sequence
        (:then_0
          (Audio|PlaySoundatLocation (.NoAmmoSound (Utilities|Struct|BreakWeaponSound_Struct (.Sounds (Utilities|Struct|BreakWeapon_Struct (Variables|Default|GetCurrentWeaponInfo))))) (Transformation|GetActorLocation) "0, 0, 0" 2.0 0.0 0.0 0 0 0))
        (:then_1
          (Utilities|FlowControl|Delay 0.2)
          (goto _label Reset))))))

(event EventTick
  (params (DeltaSeconds :type Float%20%28single-precision%29))
  ;[0 1 0.4141] Laser Sight - If Using Projectiles
  ;;[0 0.5355 1] Event Tick - If LaserSight is active, call the laser sight LineTrace to update it's location, rotation
  (if (Variables|Don'tTouch|GetIsLaserSightActive?)
    (CallFunction|LaserSightLineTrace)))

(event EventBeginPlay
  ;[0.9922 0 1] Begin Event
  (bind _returnvalue (Utilities|GetDataTableRow "/Game/Blueprints/Data/Weapons/Weapon_DataTable.Weapon_DataTable" (Variables|Default|GetWeaponName))
    (:then
      (Variables|Default|SetCurrentWeaponInfo _returnvalue))))

(fn ConstructionScript)

(fn LaserSightLineTrace
  (bind _laserpointerarrow (Variables|Default|GetLaserPointerArrow))
  (bind _returnvalue (Transformation|GetWorldLocation _laserpointerarrow))
  ;[0.7344 1 0] LaserSight Line Trace - on every tick, updates the laserPointerMesh scale, rotation
  ;;[0 0.5355 1] Spawn a lineTrace, from the laserPointerArrow's location, in forward '5000' values
  (bind (_outhit _returnvalue_2) (Collision|LineTraceByChannel _returnvalue (+ _returnvalue (* (Math|Vector|GetForwardVector _laserpointerarrow) 5e+03)) "TraceTypeQuery1" false 0 "None"))
  ;;[0 0.5355 1] Check if the trace hits an actor (something blocks the Visibility channel)
  (if _returnvalue_2
    ;;[0 0.5355 1] On hit, update the laserSightRotation variable (used to rotate spawned projectile in the correct rotation) From TraceStart to ImpactPoint
    (Variables|Don'tTouch|SetLaserSightTraceEnd (.TraceEnd (Collision|BreakHitResult _outhit)))
    (Variables|Don'tTouch|SetLaserSightRotation (Math|Rotator|FindLookatRotation (.TraceStart (Collision|BreakHitResult _outhit)) (.ImpactPoint (Collision|BreakHitResult _outhit))))
    ;;[0 0.5355 1] Then check if there's a valid LaserSightEmitter. If there is one, set it's location to the ImpactPoint. If there isn't any, spawn one at the impact point location.
    ;; (The LaserSightEmitter is just a spark emitter at the end of the laserSight)
    (Utilities|IsValid (Variables|Default|GetLaserSightEmitter)
      (:Is%20Valid
        (Transformation|SetWorldLocation (Variables|Default|GetLaserSightEmitter) (.ImpactPoint (Collision|BreakHitResult _outhit)) true true))
      (:Is%20Not%20Valid
        (bind _returnvalue_3 (Effects|SpawnEmitteratLocation "/Game/ReactionSystemBP/DemoContent/Effects/ParticleSystems/PS_LaserPointer.PS_LaserPointer" (.ImpactPoint (Collision|BreakHitResult _outhit))))
        (Variables|Default|SetLaserSightEmitter _returnvalue_3)))
    ;;[0 0.5355 1] Setting the X scale of the LaserPointerMesh to the calculated distance's length.
    (Transformation|SetWorldScale3D (Variables|Default|GetLaserPointerMesh) (Math|Vector|MakeVector (Math|Vector|VectorLength (- (.TraceStart (Collision|BreakHitResult _outhit)) (.ImpactPoint (Collision|BreakHitResult _outhit)))) 1.0 1.0))
    (else
      ;;[0 0.5355 1] If there isn't a hit it means there's no ImpactPoint to the lineTrace, so we destroy the LaserSightEmitter(the sparks at the end of the laserSight) and set the scale of the LaserSightMesh to stretch until the end of the lineTrace (Distance between Trace Start and Trace End)
      (Variables|Don'tTouch|SetLaserSightTraceEnd (.TraceEnd (Collision|BreakHitResult _outhit)))
      (Utilities|IsValid (Variables|Default|GetLaserSightEmitter)
        (:Is%20Valid
          (Components|DestroyComponent (Variables|Default|GetLaserSightEmitter))
          (Variables|Default|SetLaserSightEmitter 0))
        (:Is%20Not%20Valid
          _))
      (Transformation|SetWorldScale3D (Variables|Default|GetLaserPointerMesh) (Math|Vector|MakeVector (Math|Vector|VectorLength (- (.TraceStart (Collision|BreakHitResult _outhit)) (.TraceEnd (Collision|BreakHitResult _outhit)))) 1.0 1.0)))))

(fn CalculateAccuracy
  (params (InVec :type Vector))
  (bind _returnvalue (Game|Player|GetPlayerPawn 0))
  (bind (_x _y _z) (Math|Vector|BreakVector InVec))
  (bind _currentweaponinfo (Variables|Default|GetCurrentWeaponInfo))
  (bind _weaponeffects (Utilities|Struct|BreakWeapon_Struct _currentweaponinfo))
  (bind _returnvalue_2 (Transformation|GetVelocity _returnvalue))
  (bind _spread (Utilities|Struct|BreakWeaponEffect_Struct _weaponeffects))
  (bind _returnvalue_3 (Math|Vector|VectorLength _returnvalue_2))
  (bind _returnvalue_4 (> _returnvalue_3 0.0))
  (bind _returnvalue_5 (* _spread 0.5))
  (bind _returnvalue_6 (select _returnvalue_4 _spread _returnvalue_5))
  (bind _returnvalue_7 (* _returnvalue_6 -1.0))
  (return (Math|Vector|MakeVector (+ _x (Math|Random|RandomFloatinRange _returnvalue_7 _returnvalue_6)) (+ _y (Math|Random|RandomFloatinRange _returnvalue_7 _returnvalue_6)) (+ _z (Math|Random|RandomFloatinRange _returnvalue_7 _returnvalue_6)))))

(fn CalculateShotVolume
  (params (Sound :type Sound%20Base%20Object%20Reference) (Pitch%20Variation :type Float%20%28single-precision%29) (Base%20Pitch :type Float%20%28single-precision%29))
  (return Sound (Math|Random|RandomFloatinRange (+ (* Pitch%20Variation -1.0) Base%20Pitch) (+ Pitch%20Variation Base%20Pitch))))