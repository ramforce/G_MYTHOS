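; Weapon component that handles firing, ammo and reloading for the equipped weapon, using its CurrentWeaponInfo struct.
; Tick drives automatic fire while the trigger is held, and HandleGunInput feeds single shots into the same path.
; A Gate paces shots, reopening after the fire-rate delay, while bursts loop past it.
; Delayed reloads move reserve rounds into the clip, with perfect reloads adding SpecialAmmo; AmmoPrompt and accuracy logic are unfinished.
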(event Custom|Equip%20New%20Weapon
  (params (WeaponReference :type BP%20Weapon%20Ranged%20Master%20Object%20Reference))
  (bind _output_get (Variables|Default|SetWeaponReference WeaponReference))
  (Variables|Default|SetTempBurstLength (.BurstLength (Utilities|Struct|BreakWeapon_Struct (Variables|/Game/Blueprints/Weapons/BP_Weapon_Ranged_Master.BP_Weapon_Ranged_Master_C|GetCurrentWeaponInfo _output_get)))))

(event Custom|Shoot)

(event Custom|Weapon%20Tick
  (bind _weaponreference (Variables|Default|GetWeaponReference))
  (bind _weaponreference_2 (Variables|Default|GetWeaponReference))
  (bind _canshoot_ (Variables|States|GetcanShoot?))
  (bind _currentweaponinfo (Variables|/Game/Blueprints/Weapons/BP_Weapon_Ranged_Master.BP_Weapon_Ranged_Master_C|GetCurrentWeaponInfo _weaponreference_2))
  (bind _currentweaponinfo_2 (Variables|/Game/Blueprints/Weapons/BP_Weapon_Ranged_Master.BP_Weapon_Ranged_Master_C|GetCurrentWeaponInfo _weaponreference))
  (bind (_weaponname _burstlength _burstinterval _firerate) (Utilities|Struct|BreakWeapon_Struct _currentweaponinfo_2))
  (bind (_weaponname_2 _weaponammo _weaponeffects _burstlength_2 _burstinterval_2 _firerate_2 _automatic) (Utilities|Struct|BreakWeapon_Struct _currentweaponinfo))
  (bind _clipammo (Utilities|Struct|BreakWeaponAmmo_Struct _weaponammo))
  (bind _returnvalue (> _clipammo 0))
  (bind _returnvalue_2 (and _canshoot_ _returnvalue))
  ;[0.07812 1 0] Handle Gun Input
  ;;[1 0.6563 0] Automatic Fire
  (Utilities|IsValid _weaponreference_2
    (:Is%20Valid
      (if (and (.Automatic (Utilities|Struct|BreakWeapon_Struct (Variables|/Game/Blueprints/Weapons/BP_Weapon_Ranged_Master.BP_Weapon_Ranged_Master_C|GetCurrentWeaponInfo _weaponreference_2))) (Variables|States|GettriggerHeld?))
        (if _returnvalue_2
          (Utilities|FlowControl|Sequence
            (:then_0
              (Utilities|FlowControl|Gate false :!label _label
                (:Exit
                  (if _returnvalue_2
                    (Default|FireWeapon _weaponreference)
                    (bind _continueburst_ (CallFunction|UpdateAmmo))
                    (if (and _continueburst_ (> (Variables|Default|GetTempBurstLength) 1))
                      (Math|Integer|DecrementInt (Variables|Default|GetTempBurstLength)
                        (:%20%20
                          (Utilities|FlowControl|Delay _burstinterval)
                          (CallFunction|Burst)))
                      (else
                        (Utilities|FlowControl|Delay _firerate)
                        (CallFunction|ChamberRound)
                        (Variables|Default|SetTempBurstLength _burstlength)))))))
            (:then_1
              (goto _label Close)))
          (else
            ;;[0 0.5078 1] Player needs to reload
            (if _canshoot_
              (Default|EmptyGunSFX _weaponreference))))))))

(event Custom|ChamberRound
  (bind _weaponreference (Variables|Default|GetWeaponReference))
  (bind _currentweaponinfo (Variables|/Game/Blueprints/Weapons/BP_Weapon_Ranged_Master.BP_Weapon_Ranged_Master_C|GetCurrentWeaponInfo _weaponreference))
  (bind (_weaponname _burstlength _burstinterval _firerate) (Utilities|Struct|BreakWeapon_Struct _currentweaponinfo))
  ;[0.07812 1 0] Handle Gun Input
  (Utilities|FlowControl|Gate false) ; enters at Open
)

(event Custom|HandleGunInput
  (bind _weaponreference (Variables|Default|GetWeaponReference))
  (bind _weaponreference_2 (Variables|Default|GetWeaponReference))
  (bind _canshoot_ (Variables|States|GetcanShoot?))
  (bind _currentweaponinfo (Variables|/Game/Blueprints/Weapons/BP_Weapon_Ranged_Master.BP_Weapon_Ranged_Master_C|GetCurrentWeaponInfo _weaponreference_2))
  (bind _currentweaponinfo_2 (Variables|/Game/Blueprints/Weapons/BP_Weapon_Ranged_Master.BP_Weapon_Ranged_Master_C|GetCurrentWeaponInfo _weaponreference))
  (bind (_weaponname _burstlength _burstinterval _firerate) (Utilities|Struct|BreakWeapon_Struct _currentweaponinfo_2))
  (bind (_weaponname_2 _weaponammo _weaponeffects _burstlength_2 _burstinterval_2 _firerate_2 _automatic) (Utilities|Struct|BreakWeapon_Struct _currentweaponinfo))
  (bind _clipammo (Utilities|Struct|BreakWeaponAmmo_Struct _weaponammo))
  (bind _returnvalue (> _clipammo 0))
  (bind _returnvalue_2 (and _canshoot_ _returnvalue))
  ;[0.07812 1 0] Handle Gun Input
  ;;[1 0.6563 0] Automatic Fire
  (Utilities|IsValid _weaponreference_2
    (:Is%20Valid
      (if (Variables|States|GetcanShoot?)
        (if _returnvalue
          (if (not _automatic)
            (if _returnvalue_2
              (Utilities|FlowControl|Sequence
                (:then_0
                  (Utilities|FlowControl|Gate false :!label _label
                    (:Exit
                      (if _returnvalue_2
                        (Default|FireWeapon _weaponreference)
                        (bind _continueburst_ (CallFunction|UpdateAmmo))
                        (if (and _continueburst_ (> (Variables|Default|GetTempBurstLength) 1))
                          (Math|Integer|DecrementInt (Variables|Default|GetTempBurstLength)
                            (:%20%20
                              (Utilities|FlowControl|Delay _burstinterval)
                              (CallFunction|Burst)))
                          (else
                            (Utilities|FlowControl|Delay _firerate)
                            (CallFunction|ChamberRound)
                            (Variables|Default|SetTempBurstLength _burstlength)))))))
                (:then_1
                  (goto _label Close)))
              (else
                ;;[0 0.5078 1] Player needs to reload
                (if _canshoot_
                  (Default|EmptyGunSFX _weaponreference)))))
          (else
            (CallFunction|AmmoPrompt true)))))))

(event Custom|Reload
  (params (perfect? :type Boolean))
  (bind _weaponreference (Variables|Default|GetWeaponReference))
  (bind _currentweaponinfo (Variables|/Game/Blueprints/Weapons/BP_Weapon_Ranged_Master.BP_Weapon_Ranged_Master_C|GetCurrentWeaponInfo _weaponreference))
  (bind (_weaponname _weaponammo _weaponeffects) (Utilities|Struct|BreakWeapon_Struct _currentweaponinfo))
  (bind (_totalammo _clipammo _clipcapacity) (Utilities|Struct|BreakWeaponAmmo_Struct _weaponammo))
  (if (and (< _clipammo _clipcapacity) (not (Variables|Default|GetisReloading)))
    (if (!= _totalammo 0)
      (Variables|Default|SetisReloading true)
      (Utilities|FlowControl|Delay (.ReloadTime (Utilities|Struct|BreakWeaponEffect_Struct _weaponeffects)))
      (CallFunction|ReloadWeapon perfect?)
      (Variables|Default|SetisReloading false)
      (else
        (CallFunction|AmmoPrompt true)))))

(event Custom|Initialise
  (params (WeaponReference :type BP%20Weapon%20Ranged%20Master%20Object%20Reference)))

(event Custom|Burst
  (bind _weaponreference (Variables|Default|GetWeaponReference))
  (bind _currentweaponinfo (Variables|/Game/Blueprints/Weapons/BP_Weapon_Ranged_Master.BP_Weapon_Ranged_Master_C|GetCurrentWeaponInfo _weaponreference))
  (bind (_weaponname _burstlength _burstinterval _firerate) (Utilities|Struct|BreakWeapon_Struct _currentweaponinfo))
  ;[0.07812 1 0] Handle Gun Input
  (if (and (Variables|States|GetcanShoot?) (> (.ClipAmmo (Utilities|Struct|BreakWeaponAmmo_Struct (.WeaponAmmo (Utilities|Struct|BreakWeapon_Struct (Variables|/Game/Blueprints/Weapons/BP_Weapon_Ranged_Master.BP_Weapon_Ranged_Master_C|GetCurrentWeaponInfo (Variables|Default|GetWeaponReference)))))) 0))
    (Default|FireWeapon _weaponreference)
    (bind _continueburst_ (CallFunction|UpdateAmmo))
    (if (and _continueburst_ (> (Variables|Default|GetTempBurstLength) 1))
      (Math|Integer|DecrementInt (Variables|Default|GetTempBurstLength)
        (:%20%20
          (Utilities|FlowControl|Delay _burstinterval)
          (CallFunction|Burst)))
      (else
        (Utilities|FlowControl|Delay _firerate)
        (CallFunction|ChamberRound)
        (Variables|Default|SetTempBurstLength _burstlength)))))

(event EventBeginPlay)

(event EventTick
  (params (DeltaSeconds :type Float%20%28single-precision%29))
  (CallFunction|WeaponTick))

(fn CalculateAccuracy
  (LocalVariables|SetAngle (Math|Random|RandomFloatinRange 0.0 3.6e+02))
  (bind _output_get (LocalVariables|SetDistanceFromCenter (Math|Random|RandomFloatinRange 0.0 0.0)))
  (return (* (Math|Trig|Cos(Degrees) (LocalVariables|GetAngle)) _output_get) (* _output_get (Math|Trig|Sin(Degrees) (LocalVariables|GetAngle)))))

(fn UpdateAmmo
  (bind _weaponreference (Variables|Default|GetWeaponReference))
  (bind _currentweaponinfo (Variables|/Game/Blueprints/Weapons/BP_Weapon_Ranged_Master.BP_Weapon_Ranged_Master_C|GetCurrentWeaponInfo _weaponreference))
  (bind (_weaponname _weaponammo _weaponeffects _burstlength _burstinterval _firerate _automatic _holstersocket _equipsockets _weaponactionanim _weaponanimspeed _shotdecal _sounds _muzzleflare _weaponshakeclass) (Utilities|Struct|BreakWeapon_Struct _currentweaponinfo))
  (bind (_totalammo _clipammo _clipcapacity _infinite_) (Utilities|Struct|BreakWeaponAmmo_Struct _weaponammo))
  (bind _result (Math|Integer|DecrementInt _clipammo)
    (:%20%20
      (bind _structout (Utilities|Struct|SetmembersinWeapon_Struct _currentweaponinfo _weaponname (Utilities|Struct|MakeWeaponAmmo_Struct _totalammo _result _clipcapacity _infinite_) _weaponeffects _burstlength _burstinterval _firerate _automatic _holstersocket _equipsockets _weaponactionanim _weaponanimspeed _shotdecal _sounds _muzzleflare _weaponshakeclass))
      (CallFunction|AmmoPrompt (> (/ (Math|Conversions|ToFloat(Integer) (.clipcapacity (.WeaponAmmo (Utilities|Struct|BreakWeapon_Struct _structout)))) (Math|Conversions|ToFloat(Integer) (.clipammo (.WeaponAmmo (Utilities|Struct|BreakWeapon_Struct _structout))))) 2.5))
      (return (not (< _result 1))))))

(fn BurstFire)

(fn AmmoPrompt
  (params (Prompt? :type Boolean))
  ;[0 0.6719 1] add branch for no ammo
  (if true
    _))

(fn ReloadWeapon
  (params (perfect? :type Boolean))
  (bind _weaponreference (Variables|Default|GetWeaponReference))
  (bind _currentweaponinfo (Variables|/Game/Blueprints/Weapons/BP_Weapon_Ranged_Master.BP_Weapon_Ranged_Master_C|GetCurrentWeaponInfo _weaponreference))
  (bind (_weaponname _weaponammo _weaponeffects _burstlength _burstinterval _firerate _automatic _holstersocket _equipsockets _weaponactionanim _weaponanimspeed _shotdecal _sounds _muzzleflare _weaponshakeclass) (Utilities|Struct|BreakWeapon_Struct _currentweaponinfo))
  (while (and (!= (.totalammo _weaponammo) 0) (!= (.clipammo _weaponammo) (.clipcapacity _weaponammo)))
    (Utilities|Struct|SetmembersinWeapon_Struct _currentweaponinfo _weaponname (Utilities|Struct|MakeWeaponAmmo_Struct (- (.totalammo _weaponammo) 1) (+ (.clipammo _weaponammo) 1) (.clipcapacity _weaponammo) (.infinite? _weaponammo)) _weaponeffects _burstlength _burstinterval _firerate _automatic _holstersocket _equipsockets _weaponactionanim _weaponanimspeed _shotdecal _sounds _muzzleflare _weaponshakeclass)
    (if perfect?
      (Math|Integer|IncrementInt (Variables|Default|GetSpecialAmmo)))))