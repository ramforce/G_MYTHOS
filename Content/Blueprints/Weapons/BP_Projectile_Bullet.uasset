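; Bullet projectile that damages actors it hits, feeding hit data to their reaction component.
; On a blocking Hit with a non-owner, it prints the actor's name, then requires a BP_ReactionComponent, which receives the bone and component before ApplyDamage.
; Overlap handlers are empty; their alternative logic, including a sphere trace for bone data, is disconnected.
; DestroyActor and debug visibility are also unwired, so this graph never destroys the bullet.
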(event OnComponentBeginOverlap(CollisionSphere)
  (params (OverlappedComponent :type Primitive%20Component%20Object%20Reference) (OtherActor :type Actor%20Object%20Reference) (OtherComp :type Primitive%20Component%20Object%20Reference) (OtherBodyIndex :type Integer) (bFromSweep :type Boolean) (SweepResult :type Hit%20Result%20Structure%20%28by%20ref%29))
  ;[0 1 0.7656] OnComponentBeginOverlap - When projectile overlaps with any actor. (CollisionResponse of hit actor must be set to "Overlap")
  ;;[0 0.5355 1] On Overlap, as a safety check, make sure the projectile doesn't overlap with the owner actor.
)

(event Custom|OnComponentBeginOverlap%28CollisionSphere%29Copy
  (params (OverlappedComponent :type Primitive%20Component%20Object%20Reference) (OtherActor :type Actor%20Object%20Reference) (OtherComp :type Primitive%20Component%20Object%20Reference) (OtherBodyIndex :type Integer) (bFromSweep :type Boolean) (SweepResult :type Hit%20Result%20Structure%20%28by%20ref%29))
  ;[1 0 0.1875] OnComponentBeginOverlap - When projectile overlaps with any actor (w/ TracingMethod)
  ;;[0 0.5355 1] On Overlap, as a safety check, make sure the projectile doesn't overlap with the owner actor.
)

(event EventTick
  (params (DeltaSeconds :type Float%20%28single-precision%29)))

(event Collision|EventHit
  (params (MyComp :type Primitive%20Component%20Object%20Reference) (Other :type Actor%20Object%20Reference) (OtherComp :type Primitive%20Component%20Object%20Reference) (bSelfMoved :type Boolean) (HitLocation :type Vector :default "0, 0, 0") (HitNormal :type Vector :default "0, 0, 0") (NormalImpulse :type Vector :default "0, 0, 0") (Hit :type Hit%20Result%20Structure%20%28by%20ref%29))
  (bind (_bblockinghit _binitialoverlap _time _distance _location _impactpoint _normal _impactnormal _physmat _hitactor _hitcomponent _hitbonename) (Collision|BreakHitResult Hit))
  (bind _returnvalue (Actor|GetComponentbyClass _hitactor "/Game/ReactionSystemBP/Blueprints/Components/BP_ReactionComponent.BP_ReactionComponent_C"))
  ;[0 0.4375 1] EventHit - When projectile hits any actor. (CollisionResponse of HitActor must be set to "Block")
  ;;[0 0.5355 1] On Event Hit, as a safety check, make sure the projectile doesn't hit the owner actor.
  (if (and (!= Other (Components|GetOwner)) (!= Other 0))
    ;;[1 0 0] IMPORTANT - Check if the hit actor has a ReactionComponent, and calling the UpdateHitInformation  BEFORE applying damage. This updates the "BoneToReact" and the "HitComponent" on the ReactionComponent.
    (Development|PrintString (Utilities|GetDisplayName _hitactor))
    (Utilities|IsValid _returnvalue
      (:Is%20Valid
        (Default|ServerUpdateHitInformation _returnvalue _hitbonename _hitcomponent)
        ;;[0 0.5355 1] After Updating the hit information, start applying the damage to the hit character, and destroying the projectile actor (self).
        (Game|Damage|ApplyDamage _hitactor (Variables|Default|GetProjectileDamage) 0 0))
      (:Is%20Not%20Valid))))

(event EventBeginPlay
  (bind _debuggingon_ (Class|BPIDeveloperOptions|IsDebuggingOn?(Message) (Game|GetPlayerCharacter 0))))

(fn ConstructionScript)