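; Master melee weapon Blueprint that damages characters carrying BP_ReactionComponent, using either trace-based or collision-based hit detection.
; In trace mode, Start/StopMeleeAttack gate per-tick sphere traces along player 0's control rotation, limited to one hit per attack.
; In collision mode, HitCollision overlaps deal damage, with copied handler variants adding a sphere trace for bone names and a hitbox fallback.
; Each path updates the reaction component's hit information before applying damage.
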(event OnComponentBeginOverlap(HitCollision)
  (params (OverlappedComponent :type Primitive%20Component%20Object%20Reference) (OtherActor :type Actor%20Object%20Reference) (OtherComp :type Primitive%20Component%20Object%20Reference) (OtherBodyIndex :type Integer) (bFromSweep :type Boolean) (SweepResult :type Hit%20Result%20Structure%20%28by%20ref%29))
  (bind _returnvalue (Actor|GetComponentbyClass OtherActor "/Game/ReactionSystemBP/Blueprints/Components/BP_ReactionComponent.BP_ReactionComponent_C"))
  ;[1 1 1] HitCollision BeginOverlap - Dealing damage to character with collision based weapons.
  ;;[0 0.5355 1] OnOverlap - Check if the CollisionType is collision based (make sure not to deal damage with trace based weapons)
  (switch Utilities|FlowControl|Switch|SwitchonE_WeaponCollisionTypes (Variables|WeaponSetup|GetWeaponCollisionType)
    (:NewEnumerator1
      ;;[0 0.5355 1] Check if the overlapping actor is not the weapon or the owner (character)
      (if (!= OtherActor (Components|GetOwner))
        (if (!= self OtherActor)
          ;;[1 0 0] IMPORTANT - Calling the UpdateHitInformation  BEFORE applying damage. This updates the "BoneToReact" and the "HitComponent" on the ReactionComponent. Notice - in this case, the TracedBone will be 'None' because Overlap events can't recognise hit bones. The system will use the HitComponent.
          (Utilities|IsValid _returnvalue
            (:Is%20Valid
              (Default|ServerUpdateHitInformation _returnvalue "None" OtherComp)
              ;;[0 0.5355 1] Then after the HitInformation has been updated, we just apply the damage to the overlapping character.
              (Game|Damage|ApplyDamage OtherActor (.WeaponDamage (Utilities|Struct|BreakS_WeaponInfo (Variables|WeaponSetup|GetWeaponInfo))) 0 (Components|GetOwner)))))))))

(event Custom|OnComponentBeginOverlap%28HitCollision%29Copy2
  (params (OverlappedComponent :type Primitive%20Component%20Object%20Reference) (OtherActor :type Actor%20Object%20Reference) (OtherComp :type Primitive%20Component%20Object%20Reference) (OtherBodyIndex :type Integer) (bFromSweep :type Boolean) (SweepResult :type Hit%20Result%20Structure%20%28by%20ref%29))
  (bind _returnvalue (Actor|GetComponentbyClass OtherActor "/Game/ReactionSystemBP/Blueprints/Components/BP_ReactionComponent.BP_ReactionComponent_C"))
  (bind _defaultsceneroot (Variables|Default|GetDefaultSceneRoot))
  (bind _returnvalue_2 (Transformation|GetWorldLocation _defaultsceneroot))
  ;[1 1 1] HitCollision BeginOverlap - Dealing damage to character with collision based weapons and Traces, If the characters have hitboxes.
  ;;[0 0.5355 1] OnOverlap - Check if the CollisionType is collision based (make sure not to deal damage with trace based weapons)
  (switch Utilities|FlowControl|Switch|SwitchonE_WeaponCollisionTypes (Variables|WeaponSetup|GetWeaponCollisionType)
    (:NewEnumerator1
      ;;[0 0.5355 1] Check if the overlapping actor is not the weapon or the owner (character)
      (if (!= OtherActor (Components|GetOwner))
        (if (!= self OtherActor)
          ;;[1 1 1] By playing a SphereTrace(Or any kind of trace) when the weapon overlaps with a character will make sure that if the trace hits the character we can call the UpdateHitInformation event directly with the HitBone and HitComponent from the HitResult of the trace.
          (bind (_outhit _returnvalue_3) (Collision|SphereTraceForObjects _returnvalue_2 _returnvalue_2 1e+01 (Utilities|Array|MakeArray "ObjectTypeQuery3") false (Utilities|Array|MakeArray (Components|GetOwner) self) "ForDuration"))
          (if _returnvalue_3
            ;;[1 0 0] IMPORTANT - Calling the UpdateHitInformation  BEFORE applying damage. This updates the "BoneToReact" and the "HitComponent" on the ReactionComponent. Notice - in this case, the TracedBone will be the HitResult's "HitBoneName"
            ;; This way the Character will not have to be fully equipped with HitBoxes to deal damage.
            (Utilities|IsValid (Actor|GetComponentbyClass (.HitActor (Collision|BreakHitResult _outhit)) "/Game/ReactionSystemBP/Blueprints/Components/BP_ReactionComponent.BP_ReactionComponent_C")
              (:Is%20Valid
                (Default|ServerUpdateHitInformation (Actor|GetComponentbyClass (.HitActor (Collision|BreakHitResult _outhit)) "/Game/ReactionSystemBP/Blueprints/Components/BP_ReactionComponent.BP_ReactionComponent_C") (.HitBoneName (Collision|BreakHitResult _outhit)) (.HitComponent (Collision|BreakHitResult _outhit)))
                ;;[0 0.5355 1] Then after the HitInformation has been updated, we just apply the damage to the HitActor of the sphereTrace.
                (Game|Damage|ApplyDamage (.HitActor (Collision|BreakHitResult _outhit)) (.WeaponDamage (Utilities|Struct|BreakS_WeaponInfo (Variables|WeaponSetup|GetWeaponInfo))) 0 (Components|GetOwner))))
            (else
              ;;[1 0 0] IMPORTANT - If the sphereTrace doesn't find a HitResult for some reason (Should always have, because the sphere trace is called on Overlap, so the weapon should be overlapping with the character)
              ;; If there isn't a hit, we can use the OtherComponent of the OverlapEvent, if there are Hitboxes set up for the character. This way, even if the SphereTrace fails, the damage will still be dealt using the Hitbox.
              (Utilities|IsValid _returnvalue
                (:Is%20Valid
                  (Default|ServerUpdateHitInformation _returnvalue "None" OtherComp)
                  ;;[0 0.5355 1] Then after the HitInformation has been updated, we just apply the damage to the overlapping character. using the OtherActor from the Overlap Event
                  (Game|Damage|ApplyDamage OtherActor (.WeaponDamage (Utilities|Struct|BreakS_WeaponInfo (Variables|WeaponSetup|GetWeaponInfo))) 0 (Components|GetOwner)))))))))))

(event Custom|StartMeleeAttack
  ;[1 1 1] StartMeleeAttack - called from CharacterBP (BP_ExampleReactionCharacter) when the player starts a melee attack. If the CollisionType is set to TraceBased, this will set the "ShouldDrawTraces" to true - so event tick will continously play sphere traces while the player is attacking.
  (switch Utilities|FlowControl|Switch|SwitchonE_WeaponCollisionTypes (Variables|WeaponSetup|GetWeaponCollisionType)
    (:NewEnumerator0
      (Variables|Don'tTouch|SetShouldDrawTraces? true))))

(event Custom|StopMeleeAttack
  ;[1 1 1] StopMeleeAttack - called when AnimNotify "StopAttacking" is called on the melee AnimMontages, reverts everything to their default values.
  (Variables|Don'tTouch|SetShouldDrawTraces? false)
  (Variables|Don'tTouch|SetDamageDealt? false))

(event Custom|OnComponentBeginOverlap%28HitCollision%29Copy
  (params (OverlappedComponent :type Primitive%20Component%20Object%20Reference) (OtherActor :type Actor%20Object%20Reference) (OtherComp :type Primitive%20Component%20Object%20Reference) (OtherBodyIndex :type Integer) (bFromSweep :type Boolean) (SweepResult :type Hit%20Result%20Structure%20%28by%20ref%29))
  (bind _defaultsceneroot (Variables|Default|GetDefaultSceneRoot))
  (bind _returnvalue (Transformation|GetWorldLocation _defaultsceneroot))
  ;[1 1 1] HitCollision BeginOverlap - Dealing damage to character with collision based weapons and Traces.
  ;;[0 0.5355 1] OnOverlap - Check if the CollisionType is collision based (make sure not to deal damage with trace based weapons)
  (switch Utilities|FlowControl|Switch|SwitchonE_WeaponCollisionTypes (Variables|WeaponSetup|GetWeaponCollisionType)
    (:NewEnumerator1
      ;;[0 0.5355 1] Check if the overlapping actor is not the weapon or the owner (character)
      (if (!= OtherActor (Components|GetOwner))
        (if (!= self OtherActor)
          ;;[1 1 1] By playing a SphereTrace(Or any kind of trace) when the weapon overlaps with a character will make sure that if the trace hits the character we can call the UpdateHitInformation event directly with the HitBone and HitComponent from the HitResult of the trace.
          (bind (_outhit _returnvalue_2) (Collision|SphereTraceForObjects _returnvalue _returnvalue 1e+01 (Utilities|Array|MakeArray "ObjectTypeQuery3") false (Utilities|Array|MakeArray (Components|GetOwner) self) "ForDuration"))
          (if _returnvalue_2
            ;;[1 0 0] IMPORTANT - Calling the UpdateHitInformation  BEFORE applying damage. This updates the "BoneToReact" and the "HitComponent" on the ReactionComponent. Notice - in this case, the TracedBone will be the HitResult's "HitBoneName"
            ;; This way the Character will not have to be fully equipped with HitBoxes to deal damage.
            (Utilities|IsValid (Actor|GetComponentbyClass (.HitActor (Collision|BreakHitResult _outhit)) "/Game/ReactionSystemBP/Blueprints/Components/BP_ReactionComponent.BP_ReactionComponent_C")
              (:Is%20Valid
                (Default|ServerUpdateHitInformation (Actor|GetComponentbyClass (.HitActor (Collision|BreakHitResult _outhit)) "/Game/ReactionSystemBP/Blueprints/Components/BP_ReactionComponent.BP_ReactionComponent_C") (.HitBoneName (Collision|BreakHitResult _outhit)) (.HitComponent (Collision|BreakHitResult _outhit)))
                ;;[0 0.5355 1] Then after the HitInformation has been updated, we just apply the damage to the overlapping character.
                (Game|Damage|ApplyDamage (.HitActor (Collision|BreakHitResult _outhit)) (.WeaponDamage (Utilities|Struct|BreakS_WeaponInfo (Variables|WeaponSetup|GetWeaponInfo))) 0 (Components|GetOwner))))))))))

(event EventTick
  (params (DeltaSeconds :type Float%20%28single-precision%29))
  ;[1 1 1] Event Tick - If ShouldDrawTraces == true, play the AttackingSphereTrace function repeatedly, to check for a hit.
  (if (Variables|Don'tTouch|GetShouldDrawTraces?)
    (CallFunction|AttackingSphereTrace)))

(fn ConstructionScript)

(fn AttackingSphereTrace
  (bind _returnvalue (Transformation|GetActorLocation))
  ;[1 1 1] Attacking Sphere Trace - Called when using melee attacks with Trace based mode.
  ;;[0 0.5355 1] SphereTraceByChannel, starting from the location of the melee weapon, ending at "WeaponTraceLength" amounts in the forward direction, ignoring the weapon and the owner of the weapon (character)
  (bind _debuggingon_ (Class|BPIDeveloperOptions|IsDebuggingOn?(Message) (Components|GetOwner)))
  (bind (_outhit _returnvalue_2) (Collision|SphereTraceByChannel _returnvalue (+ _returnvalue (* (Math|Vector|GetForwardVector (Pawn|GetControlRotation (Game|GetPlayerController 0) :!class /Script/Engine.Controller)) (Variables|WeaponSetup|GetWeaponTraceLength))) 1e+01 "TraceTypeQuery1" false (Utilities|Array|MakeArray self (Components|GetOwner)) (select _debuggingon_ "ForDuration" "None")))
  ;;[0 0.5355 1] If there was a Hit (an actor - character - blocks the sphere trace ) check if the weapon already dealt damage with a sphere trace.
  (if _returnvalue_2
    (if (not (Variables|Don'tTouch|GetDamageDealt?))
      ;;[1 0 0] IMPORTANT - Calling the UpdateHitInformation  BEFORE applying damage. This updates the "BoneToReact" and the "HitComponent" on the ReactionComponent.
      (Utilities|IsValid (Actor|GetComponentbyClass (.HitActor (Collision|BreakHitResult _outhit)) "/Game/ReactionSystemBP/Blueprints/Components/BP_ReactionComponent.BP_ReactionComponent_C")
        (:Is%20Valid
          (Default|ServerUpdateHitInformation (Actor|GetComponentbyClass (.HitActor (Collision|BreakHitResult _outhit)) "/Game/ReactionSystemBP/Blueprints/Components/BP_ReactionComponent.BP_ReactionComponent_C") (.HitBoneName (Collision|BreakHitResult _outhit)) (.HitComponent (Collision|BreakHitResult _outhit)))
          ;;[0 0.5355 1] After the Hit Information has been updated, apply damage with the damage that has been set up in the "WeaponInfo" and set the DamageDealt? to true, meaning other traces will not deal damage to the actor.
          (Game|Damage|ApplyDamage (.HitActor (Collision|BreakHitResult _outhit)) (.WeaponDamage (Utilities|Struct|BreakS_WeaponInfo (Variables|WeaponSetup|GetWeaponInfo))) 0 0)
          (Variables|Don'tTouch|SetDamageDealt? true))))))