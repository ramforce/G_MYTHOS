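; BP_TSHS_PlayerController is a player controller that handles pawn possession and player respawn requests.
; Pressing F without a valid controlled pawn calls RequestGMRespawn, which, only on authority, asks BP_TSHS_GameMode to respawn this controller through RPCPlayerRespawn.
; RPCPossessPawn and RPCDestroyActor, grouped as server functions, possess a given pawn and destroy a given actor.
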(event Custom|RPC%20Possess%20Pawn
  (params (Pawn :type Pawn%20Object%20Reference))
  ;[1 0 0.0331] Server functions
  (Pawn|Possess Pawn))

(event Custom|Request%20GM%20Respawn
  (bind _returnvalue (Game|GetGameMode))
  ;[1 0 0.0331] Server functions
  (Networking|SwitchHasAuthority
    (:Authority
      (Utilities|IsValid _returnvalue
        (:Is%20Valid
          (bind _asbp_tshs_game_mode (Utilities|Casting|CastToBP_TSHS_GameMode _returnvalue))
          (Utilities|IsValid _asbp_tshs_game_mode
            (:Is%20Valid
              (Default|RPCPlayerRespawn _asbp_tshs_game_mode self))))))))

(event Custom|RPC%20DestroyActor
  (params (Target :type Actor%20Object%20Reference))
  ;[1 0 0.0331] Server functions
  (Actor|DestroyActor Target))

(event EventBeginPlay
  ;[1 0 0.0331] Server functions
)

(event Input|KeyboardEvents|F
  (params (Key :type Key%20Structure))
  ;[1 0 0.0331] Server functions
  ;;[0 0 0] InputAction Respawn
  (:Pressed
    (Utilities|IsValid (Pawn|GetControlledPawn self)
      (:Is%20Not%20Valid
        (CallFunction|RequestGMRespawn)))))

(fn ConstructionScript)