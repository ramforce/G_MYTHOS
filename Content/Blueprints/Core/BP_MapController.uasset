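; Player-controlled map pawn that moves around the map view and lets the player cycle through, focus on and possess BP_MythosCharacter_Master characters.
; An actor array holds itself plus every character; Q/E or click override blend the camera between entries, and Space possesses the selection.
; IsSwitchingView gates input during blends, while a timeline and material parameter collection drive a positional outline effect.
; RegainMapControl repossesses the pawn and rebuilds the roster HUD.
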(event Custom|SelectCharacter
  (bind _returnvalue (Game|GetPlayerController 0))
  (bind _actorarray (Variables|Default|GetActorArray))
  (bind _currentcharacterindex (Variables|Default|GetCurrentCharacterIndex))
  (bind _output (Utilities|Array|Get(acopy) _actorarray _currentcharacterindex))
  ;[0 0.1797 1] Select Character
  (if (not (Variables|Default|GetisSwitchingView?))
    (Utilities|Casting|CastToBP_MapController _output
      (:CastFailed
        (Utilities|IsValid _output
          (:Is%20Valid
            (Variables|Default|SetisSwitchingView? true)
            (Game|Player|SetViewTargetwithBlend _returnvalue _output 2.0 "VTBlend_Cubic" 0.0 false)
            (bind _asbp_mythos_character_master (Utilities|Casting|CastToBP_MythosCharacter_Master _output))
            (Pawn|Possess _returnvalue _asbp_mythos_character_master)
            (Default|InitialiseControl _asbp_mythos_character_master)
            (Widget|RemovefromParent (Variables|Default|GetMapHUD))
            (Variables|Default|SetisSwitchingView? true)))))))

(event Custom|NextCharacter
  (params (isPrevious? :type Boolean))
  (bind _returnvalue (Game|GetPlayerController 0))
  (bind _actorarray (Variables|Default|GetActorArray))
  ;[0.8516 0 1] Next Character
  (bind _output_get (Variables|Default|SetCurrentCharacterIndex (CallFunction|FindNextCharacterIndex _actorarray isPrevious?)))
  (Utilities|IsValid (Utilities|Array|Get(acopy) _actorarray _output_get)
    (:Is%20Valid
      (bind _asbp_mythos_character_master (Utilities|Casting|CastToBP_MythosCharacter_Master (Utilities|Array|Get(acopy) _actorarray _output_get))
        (:then
          (Game|Player|SetViewTargetwithBlend _returnvalue (Utilities|Array|Get(acopy) _actorarray _output_get) 1.5 "VTBlend_Cubic" 0.0 false)
          (Default|RefreshRoster (Variables|Default|GetMapHUD) (Variables|/Game/Blueprints/BattleEventSystem/BPC_BattleEventComponent.BPC_BattleEventComponent_C|GetCharacterInfo (Variables|/Game/Blueprints/Core/BP_MythosCharacter_Master.BP_MythosCharacter_Master_C|GetBPC_BattleEventComponent _asbp_mythos_character_master)))
          (Utilities|FlowControl|Delay 1.5)
          (CallFunction|PostPro (Utilities|Array|Get(acopy) _actorarray _output_get) 0.1)
          (Variables|Default|SetisSwitchingView? false))
        (:CastFailed
          (Game|Player|SetViewTargetwithBlend _returnvalue (Utilities|Array|Get(acopy) _actorarray _output_get) 1.5 "VTBlend_Cubic" 0.0 false)
          (Utilities|FlowControl|Delay 1.5)
          (CallFunction|PostPro (Utilities|Array|Get(acopy) _actorarray _output_get) 1.0)
          (Variables|Default|SetisSwitchingView? false))))))

(event Custom|PostPro
  (params (Target :type Actor%20Object%20Reference) (NewTime :type Float%20%28single-precision%29))
  ;[1 0 0.1406] Post Processing FX
  (Utilities|IsValid Target
    (:Is%20Valid
      (Rendering|Material|SetVectorParameterValue "/Game/PostProccess/PC_Outline.PC_Outline" "Position" (Math|Conversions|ToLinearColor(Vector) (Transformation|GetActorLocation Target)) :!class /Script/Engine.KismetMaterialLibrary)
      (if (== Target self)
        (bind _newtrack_0 (Timeline|Timeline_0 ReverseFromEnd)
          (:Update
            (Rendering|Material|SetScalarParameterValue "/Game/PostProccess/PC_Outline.PC_Outline" "Radius" _newtrack_0 :!class /Script/Engine.KismetMaterialLibrary)))
        (else
          (Timeline|Timeline_0 PlayFromStart))))))

(event Custom|ClickOverride
  (params (InputObject :type Actor%20Object%20Reference))
  (bind _actorarray (Variables|Default|GetActorArray))
  (bind _returnvalue (Utilities|Array|FindItem _actorarray InputObject))
  ;[1 0 0.4922] Click Actor Override
  (if (not (or (== _returnvalue (Variables|Default|GetCurrentCharacterIndex)) (Variables|Default|GetisSwitchingView?)))
    (Utilities|IsValid InputObject
      (:Is%20Valid
        (Variables|Default|SetisSwitchingView? true)
        (Variables|Default|SetCurrentCharacterIndex _returnvalue)
        (bind _asbp_mythos_character_master (Utilities|Casting|CastToBP_MythosCharacter_Master InputObject))
        (Game|Player|SetViewTargetwithBlend (Game|GetPlayerController 0) _asbp_mythos_character_master 2.0 "VTBlend_Cubic" 0.0 false)
        (Default|RefreshRoster (Variables|Default|GetMapHUD))
        (Utilities|FlowControl|Delay 2.0)
        (CallFunction|PostPro InputObject 0.1)
        (Variables|Default|SetisSwitchingView? false)))))

(event EventBeginPlay
  (CallFunction|InitialiseMap))

(event Input|AxisEvents|InputAxisMoveForward
  (params (AxisValue :type Float%20%28single-precision%29))
  ;[0.5703 1 0] Map Controls
  (if (CallFunction|MovementCheck)
    (Pawn|Input|AddMovementInput (Math|Vector|GetForwardVector (Pawn|GetControlRotation :!class /Script/Engine.Pawn)) AxisValue false)))

(event Input|AxisEvents|InputAxisMoveRight
  (params (AxisValue :type Float%20%28single-precision%29))
  ;[0.5703 1 0] Map Controls
  (if (CallFunction|MovementCheck)
    (Pawn|Input|AddMovementInput (Math|Vector|GetRightVector (Pawn|GetControlRotation :!class /Script/Engine.Pawn)) AxisValue false)))

(event Input|KeyboardEvents|Q
  (params (Key :type Key%20Structure))
  ;[1 0.9375 0] Switch Character Viewpoint
  (:Pressed
    (if (not (Variables|Default|GetisSwitchingView?))
      (Variables|Default|SetisSwitchingView? true)
      (CallFunction|NextCharacter false))))

(event Input|KeyboardEvents|E
  (params (Key :type Key%20Structure))
  ;[1 0.9375 0] Switch Character Viewpoint
  (:Pressed
    (if (not (Variables|Default|GetisSwitchingView?))
      (Variables|Default|SetisSwitchingView? true)
      (CallFunction|NextCharacter true))))

(event Input|KeyboardEvents|SpaceBar
  (params (Key :type Key%20Structure))
  ;[1 0.9375 0] Switch Character Viewpoint
  (:Pressed
    (CallFunction|SelectCharacter)))

(fn ConstructionScript)

(fn FindNextCharacterIndex
  (params (TargetArray :type Array%20of%20Actor%20Object%20References) (IsPrevious? :type Boolean))
  (bind _returnvalue (Utilities|Array|LastIndex TargetArray))
  (bind _currentcharacterindex (Variables|Default|GetCurrentCharacterIndex))
  (bind _returnvalue_2 (- _currentcharacterindex 1))
  (bind _returnvalue_3 (+ _currentcharacterindex 1))
  (return (Math|Integer|SelectInt (Math|Integer|SelectInt _returnvalue _returnvalue_2 (< _returnvalue_2 0)) (Math|Integer|SelectInt 0 _returnvalue_3 (< _returnvalue _returnvalue_3)) IsPrevious?)))

(fn InitialiseMap
  (bind _returnvalue (Game|GetPlayerController 0))
  (bind _actorarray (Variables|Default|GetActorArray))
  (Variables|Default|SetCurrentCharacterIndex 0)
  (Variables|Default|SetisSwitchingView? false)
  (CallFunction|PostPro 0 0.0)
  (Utilities|Array|Add _actorarray self)
  (bind _outactors (Actor|GetAllActorsOfClass "/Game/Blueprints/Core/BP_MythosCharacter_Master.BP_MythosCharacter_Master_C"))
  (Utilities|Array|AppendArray _actorarray _outactors)
  (Utilities|IsValid (Variables|Default|GetMapHUD)
    (:Is%20Valid
      _)
    (:Is%20Not%20Valid
      (bind _returnvalue_2 (UserInterface|CreateWidget "/Game/UserInterface/W_MapCamera-HUD.W_MapCamera-HUD_C" _returnvalue))
      (bind _output_get (Variables|Default|SetMapHUD _returnvalue_2))))
  (UserInterface|Viewport|AddtoViewport _output_get 0)
  (Default|Initialise _output_get _actorarray)
  (Input|SetInputModeGameandUI _returnvalue _output_get "DoNotLock" false)
  (Variables|/Script/Engine.PlayerController|SetbShowMouseCursor _returnvalue true))

(fn MovementCheck
  (return (Math|Boolean|NORBoolean (Variables|Default|GetisSwitchingView?) (!= (Utilities|Array|Get(acopy) (Variables|Default|GetActorArray) (Variables|Default|GetCurrentCharacterIndex)) self))))

(fn RegainMapControl
  (bind _returnvalue (Game|GetPlayerController 0))
  (bind _self self)
  (Utilities|Array|Clear (Variables|Default|GetActorArray))
  (Pawn|Possess _returnvalue _self)
  (Input|EnableInput _self _returnvalue)
  (Widget|Panel|ClearChildren (Variables|/Game/UserInterface/W_MapCamera-HUD.W_MapCamera-HUD_C|GetSB_RosterInfo (Variables|Default|GetMapHUD)))
  (CallFunction|InitialiseMap)
  (bind _outactors (Actor|GetAllActorsOfClass "/Game/Blueprints/Core/BP_MythosCharacter_Master.BP_MythosCharacter_Master_C"))
  (for _array_element _outactors
    (Development|SetHiddeninGame (Variables|/Game/Blueprints/Core/BP_MythosCharacter_Master.BP_MythosCharacter_Master_C|GetMapIcon _array_element) false false)))