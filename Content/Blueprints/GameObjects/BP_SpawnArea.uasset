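; BP_SpawnArea is an actor that marks a spawn area for an occupying allegiance: Ally, Enemy, Neutral or Supporting.
; The construction script labels its TextRender with the allegiance name plus "Spawn" and gives the Cube the matching material.
; The event graph holds only disabled placeholder events, so the Blueprint itself adds no runtime logic.
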(event EventBeginPlay)

(event Collision|EventActorBeginOverlap
  (params (OtherActor :type Actor%20Object%20Reference)))

(event EventTick
  (params (DeltaSeconds :type Float%20%28single-precision%29)))

(fn ConstructionScript
  (bind _occupyingalligence (Variables|Default|GetOccupyingAlligence))
  (Rendering|Components|TextRender|SetText (Variables|Default|GetTextRender) (Utilities|Text|ToText(String) (Utilities|String|Append (Utilities|String|EnumtoString _occupyingalligence) " Spawn")))
  (Rendering|Material|SetMaterial (Variables|Default|GetCube) 0 (Utilities|Select :Index _occupyingalligence :NewEnumerator1 (Variables|Default|GetAllyMaterial) :NewEnumerator4 (Variables|Default|GetEnemyMaterial) :NewEnumerator2 (Variables|Default|GetNeutralMaterial) :NewEnumerator3 (Variables|Default|GetSupportingMaterial))))