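; Basic zombie enemy NPC character with health, a melee attack montage with sound, stagger and a chase sound.
; Any damage halts movement, lowers clamped health and updates the percentage, triggering a one-time ragdoll death at zero.
; On BeginPlay it passes itself to its health bar widget.
; Player melee damage, kill-combo increment and health bar removal are disconnected, and the radial damage check does nothing.
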(event Custom|Ragdoll
  ;[1 0.75 0] Ragdoll
  (Variables|Default|SetIsDead true)
  (Physics|SetSimulatePhysics (Variables|Character|GetMesh) true)
  (Collision|SetCollisionEnabled (Variables|Collision|GetCapsuleComponent) "PhysicsOnly")
  (Pawn|Components|CharacterMovement|DisableMovement (Variables|Character|GetCharacterMovement)))

(event Custom|Chase%20Player%20Sound
  (Utilities|FlowControl|DoOnce false
    (:Completed
      (Audio|PlaySoundatLocation 0 (Transformation|GetWorldLocation (Variables|Character|GetMesh)) "0, 0, 0" 1.0 1.0 0.0 0 0 0)
      (if (== (Variables|Default|GetHealth) 0.0)
        (Utilities|TMStop3DSound)))))

(event Custom|Stagger
  ;[0 1 0.3672] Stagger
  (Class|NavMovementComponent|StopActiveMovement (Variables|Character|GetCharacterMovement))
  (Animation|Montage|MontagePlay (Components|SkeletalMesh|GetAnimInstance (Variables|Character|GetMesh)) 0 1.0 "MontageLength" 0.0 true))

(event EventBeginPlay
  ;[0 1 1] Health Bar
  (bind _asenemy_health_bar (Utilities|Casting|CastToEnemyHealthBar (UserInterface|GetUserWidgetObject (Variables|Default|GetEnemyHealthBar))))
  (bind _output_get (Variables|Default|SetEnemyHealthBarWidget _asenemy_health_bar))
  (Variables|/Game/Blueprints/AI/NPC/AI_BP/EnemyHealthBar.EnemyHealthBar_C|SetBP_NPC_Ref _output_get self))

(event Collision|EventActorBeginOverlap
  (params (OtherActor :type Actor%20Object%20Reference)))

(event EventTick
  (params (DeltaSeconds :type Float%20%28single-precision%29)))

(event Game|Damage|EventAnyDamage
  (params (Damage :type Float%20%28single-precision%29) (DamageType :type Damage%20Type%20Object%20Reference) (InstigatedBy :type Controller%20Object%20Reference) (DamageCauser :type Actor%20Object%20Reference))
  ;[1 0.8438 0] Take Damage
  (Class|NavMovementComponent|StopActiveMovement (Variables|Character|GetCharacterMovement))
  (bind _output_get (Variables|Default|SetHealth (Math|Float|Clamp(Float) (- (Variables|Default|GetHealth) Damage) 0.0 (Variables|Default|GetmaxHealth))))
  (Variables|Default|SetHealthPercentage (/ _output_get 1e+02))
  (if (Math|Float|NearlyEqual(Float) (Variables|Default|GetHealth) 0.0 1e-06)
    (Utilities|FlowControl|MultiGate false false -1
      (:Out%200
        ;;[0 1 0.4609] Increment combo count
        (CallFunction|Ragdoll)))))

(event EventMeleeAttack
  ;[0.6641 0 1] Play Melee Attack Animation
  (if (not (Variables|Default|GetIsDead))
    (Audio|PlaySoundatLocation 0 (Transformation|GetWorldLocation (Variables|Character|GetMesh)) "0, 0, 0" 1.0 1.0 0.0 0 0 0)
    (Animation|Montage|MontagePlay (Components|SkeletalMesh|GetAnimInstance (Variables|Character|GetMesh)) "/Game/Blueprints/AI/Attack_Montage.Attack_Montage" 1.0 "MontageLength" 0.0 true)))

(event Game|Damage|EventRadialDamage
  (params (DamageReceived :type Float%20%28single-precision%29) (DamageType :type Damage%20Type%20Object%20Reference) (Origin :type Vector :default "0, 0, 0") (HitInfo :type Hit%20Result%20Structure%20%28by%20ref%29) (InstigatedBy :type Controller%20Object%20Reference) (DamageCauser :type Actor%20Object%20Reference))
  ;[0 1 1] On grenade damage
  ;;[0.3828 0 1] Needs a delay to let the any damage stuff apply
  (Utilities|FlowControl|Delay 0.1)
  (if (Math|Float|NearlyEqual(Float) (Variables|Default|GetHealth) 0.0 1e-06)
    _))

(fn ConstructionScript)