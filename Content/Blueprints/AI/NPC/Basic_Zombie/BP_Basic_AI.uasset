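; AI controller for the basic zombie that runs the BT_Basic behavior tree and feeds its blackboard.
; On BeginPlay it can seed patrol looping, direction and wait time from the pawn's patrol path, gated on BP_PatrolPath being invalid.
; Perception updates pass stimuli to NoiseSenses, which maps them by array index: the first sets CanSeePlayer, the second sets IsInvestigating and TargetLocation.
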(event OnPerceptionUpdated(AIPerception)
  (params (UpdatedActors :type Array%20of%20Actor%20Object%20References))
  ;[1 1 1] Comment
  (for _array_element UpdatedActors
    (bind _info (Class|AIPerceptionComponent|GetActorsPerception (Variables|Default|GetAIPerception) _array_element))
    (CallFunction|NoiseSenses (.lastsensedstimuli _info))))

(event EventBeginPlay
  (bind _returnvalue (AI|GetBlackboard 0))
  (AI|RunBehaviorTree "/Game/Blueprints/AI/NPC/Basic_Zombie/BT_Basic.BT_Basic")
  (bind _asbp_basic_zombie (Utilities|Casting|CastToBP_Basic_Zombie (Pawn|GetControlledPawn)))
  (bind _output_get (Variables|Default|SetBasicZombie_Pawn _asbp_basic_zombie))
  (Utilities|IsValid "/Game/Blueprints/AI/NPC/AI_BP/BP_PatrolPath.BP_PatrolPath"
    (:Is%20Not%20Valid
      (AI|Components|Blackboard|SetValueasBool (AI|GetBlackboard 0) (Utilities|Name|MakeLiteralName "PathLooping") (Variables|/Game/Blueprints/AI/NPC/AI_BP/BP_PatrolPath.BP_PatrolPath_C|GetIsLooping (Variables|/Game/Blueprints/AI/NPC/Basic_Zombie/BP_Basic_Zombie.BP_Basic_Zombie_C|GetPatrolPath _output_get)))
      (Class|BlackboardComponent|SetValueasInt _returnvalue (Utilities|Name|MakeLiteralName "Direction") 1)
      (AI|Components|Blackboard|SetValueasFloat _returnvalue (Utilities|Name|MakeLiteralName "WaitTime") (Variables|/Game/Blueprints/AI/NPC/AI_BP/BP_PatrolPath.BP_PatrolPath_C|GetWaitTime (Variables|/Game/Blueprints/AI/NPC/Basic_Zombie/BP_Basic_Zombie.BP_Basic_Zombie_C|GetPatrolPath (Variables|Default|GetBasicZombie_Pawn)))))))

(fn ConstructionScript)

(fn NoiseSenses
  (params (Array :type Array%20of%20AI%20Stimulus%20Structures))
  (for (_array_element _array_index) Array
    (LocalVariables|SetLocal%20Sense _array_element)
    (switch int _array_index
      (:0
        (AI|Components|Blackboard|SetValueasBool (AI|GetBlackboard 0) (Utilities|Name|MakeLiteralName "CanSeePlayer") (.bsuccessfullysensed (LocalVariables|GetLocal%20Sense))))
      (:1
        (AI|Components|Blackboard|SetValueasBool (AI|GetBlackboard 0) (Utilities|Name|MakeLiteralName "IsInvestigating") (.bsuccessfullysensed (LocalVariables|GetLocal%20Sense)))
        (AI|Components|Blackboard|SetValueasVector (AI|GetBlackboard 0) (Utilities|Name|MakeLiteralName "TargetLocation") (.stimuluslocation (LocalVariables|GetLocal%20Sense)))))))