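; Behavior tree task that steps a zombie's patrol path index back and forth along its path points.
; It reads direction and index from the blackboard, moving forward within the BP_Basic_Zombie PatrolPath length or backward down to zero.
; At either end it flips the direction and finishes as failed without changing the index.
; A failed pawn cast on the forward branch never calls FinishExecute.
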(event EventReceiveExecuteAI
  (params (OwnerController :type AI%20Controller%20Object%20Reference) (ControlledPawn :type Pawn%20Object%20Reference))
  (bind _bb_pathindex (Variables|Default|GetBB_PathIndex))
  (bind _bb_direction (Variables|Default|GetBB_Direction))
  (bind _bb_direction_2 (Variables|Default|GetBB_Direction))
  (bind _bb_pathindex_2 (Variables|Default|GetBB_PathIndex))
  (bind _returnvalue (Class|BTFunctionLibrary|GetBlackboardValueasInt _bb_pathindex))
  (bind _returnvalue_2 (Class|BTFunctionLibrary|GetBlackboardValueasInt _bb_pathindex_2))
  (bind _returnvalue_3 (- _returnvalue 1))
  (bind _returnvalue_4 (+ _returnvalue_2 1))
  (if (== (Class|BTFunctionLibrary|GetBlackboardValueasInt (Variables|Default|GetBB_Direction)) 1)
    ;[1 1 1] If Successful Increment path
    (bind _asbp_basic_zombie (Utilities|Casting|CastToBP_Basic_Zombie ControlledPawn))
    (if (<= _returnvalue_4 (- (Utilities|Array|Length (Variables|/Game/Blueprints/AI/NPC/AI_BP/BP_PatrolPath.BP_PatrolPath_C|GetPathPoints (Variables|/Game/Blueprints/AI/NPC/Basic_Zombie/BP_Basic_Zombie.BP_Basic_Zombie_C|GetPatrolPath _asbp_basic_zombie))) 1))
      (Class|BTFunctionLibrary|SetBlackboardValueasInt _bb_direction 1)
      (Class|BTFunctionLibrary|SetBlackboardValueasInt (Variables|Default|GetBB_PathIndex) _returnvalue_4)
      (AI|BehaviorTree|FinishExecute true)
      (else
        (Class|BTFunctionLibrary|SetBlackboardValueasInt _bb_direction -1)
        (AI|BehaviorTree|FinishExecute false)))
    (else
      ;[1 1 1] If Fail Decrement Path
      (if (== (Class|BTFunctionLibrary|GetBlackboardValueasInt (Variables|Default|GetBB_Direction)) -1)
        (if (>= _returnvalue_3 0)
          (Class|BTFunctionLibrary|SetBlackboardValueasInt _bb_direction_2 -1)
          (Class|BTFunctionLibrary|SetBlackboardValueasInt (Variables|Default|GetBB_PathIndex) _returnvalue_3)
          (AI|BehaviorTree|FinishExecute true)
          (else
            (Class|BTFunctionLibrary|SetBlackboardValueasInt _bb_direction_2 1)
            (AI|BehaviorTree|FinishExecute false)))
        (else
          (AI|BehaviorTree|FinishExecute false))))))