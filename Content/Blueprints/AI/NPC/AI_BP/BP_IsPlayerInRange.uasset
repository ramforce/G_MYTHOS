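; Behavior tree service that tells an NPC's AI which attack and chase ranges player 0 falls into.
; On activation it compares the controlled pawn's distance to the player against range variables and writes Blackboard booleans for chase, sweep, melee and axe throw.
; Chase and melee are true within their ranges, while sweep is true at or beyond its range.
; The throw check uses NotThrowableRange for both bounds, so only an exact distance passes.
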(event EventReceiveActivationAI
  (params (OwnerController :type AI%20Controller%20Object%20Reference) (ControlledPawn :type Pawn%20Object%20Reference))
  (bind _returnvalue (Game|GetPlayerCharacter 0))
  (bind _returnvalue_2 (Transformation|GetDistanceTo ControlledPawn _returnvalue))
  (Class|BTFunctionLibrary|SetBlackboardValueasBool (Variables|Default|GetBK_IsInChaseRange) (<= _returnvalue_2 (Variables|Default|GetChase%20Range)))
  (Class|BTFunctionLibrary|SetBlackboardValueasBool (Variables|Default|GetBK_IsInSweepRange) (>= _returnvalue_2 (Variables|Default|GetSweepStrikeRange)))
  (Class|BTFunctionLibrary|SetBlackboardValueasBool (Variables|Default|GetBB_IsInRange) (<= _returnvalue_2 (Variables|Default|GetMeleeRange)))
  (Class|BTFunctionLibrary|SetBlackboardValueasBool (Variables|Default|GetBB_IsInThrowRange) (and (>= _returnvalue_2 (Variables|Default|GetNot%20Throwable%20Range>=)) (<= _returnvalue_2 (Variables|Default|GetNot%20Throwable%20Range<=)))))