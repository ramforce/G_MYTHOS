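; A behavior tree task that picks the world location of a zombie's current patrol point.
; It reads the path index from the blackboard, takes that point from the BP_Basic_Zombie's PatrolPath and transforms it by the path actor's transform into the blackboard path vector.
; It finishes successfully only after writing the vector; a failed cast or missing path never calls FinishExecute.
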(event EventReceiveExecuteAI
  (params (OwnerController :type AI%20Controller%20Object%20Reference) (ControlledPawn :type Pawn%20Object%20Reference))
  (bind _asbp_basic_zombie (Utilities|Casting|CastToBP_Basic_Zombie ControlledPawn))
  (bind _patrolpath (Variables|/Game/Blueprints/AI/NPC/Basic_Zombie/BP_Basic_Zombie.BP_Basic_Zombie_C|GetPatrolPath _asbp_basic_zombie)
    (:then
      (AI|BehaviorTree|SetBlackboardValueasVector (Variables|Default|GetBB_PathVector) (Math|Transform|TransformLocation (Transformation|GetActorTransform _patrolpath) (Utilities|Array|Get(acopy) (Variables|/Game/Blueprints/AI/NPC/AI_BP/BP_PatrolPath.BP_PatrolPath_C|GetPathPoints _patrolpath) (Class|BTFunctionLibrary|GetBlackboardValueasInt (Variables|Default|GetBB_PathIndex)))))
      (AI|BehaviorTree|FinishExecute true))
    (:else)))